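; BP_Kultar is the story NPC Kultar, a captive who talks, trades and moves through a scripted release sequence.
; In StoryMode, Tick drives a Scenario state machine using DoOnce gates, montages, waypoint moves and level-sequence cinematics.
; The guard goblin's death advances him, while the lever check runs every tick, allowing earlier stages to be skipped.
; Interaction plays ScenarioTalk lines and opens trade; save functions store transform and death state.
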(event OnComponentBeginOverlap(Capsule)
  (params (OverlappedComponent :type Primitive%20Component%20Object%20Reference) (OtherActor :type Actor%20Object%20Reference) (OtherComp :type Primitive%20Component%20Object%20Reference) (OtherBodyIndex :type Integer) (bFromSweep :type Boolean) (SweepResult :type Hit%20Result%20Structure%20%28by%20ref%29))
  (Utilities|Casting|CastToMonster_NBC OtherActor)
  (Utilities|FlowControl|DoOnce false
    (:Completed
      (Game|Damage|ApplyDamage OtherActor (.Value (Default|GetStatValue (Variables|Default|GetBP_Stats) "NewEnumerator4" false)) 0 self))))

(event Custom|SpeakKultar
  (params (Sound :type Sound%20Base%20Object%20Reference))
  (bind _returnvalue (Audio|SpawnSoundatLocation Sound (Transformation|GetWorldLocation (Variables|Character|GetMesh)) "0, 0, 0" 1.0 1.0 0.0 0 0))
  (Variables|Default|SetKultarTalk true)
  (Utilities|FlowControl|Delay (Variables|/Script/Engine.SoundBase|GetDuration (Variables|/Script/Engine.AudioComponent|GetSound _returnvalue)))
  (Variables|Default|SetKultarTalk false))

(event Custom|SpecScenario
  (switch int (Variables|Default|GetScenario_Talk)
    (:1
      (CallFunction|SpeakKultar "/Game/NPC/KultarNPC/Song/lookwell/Kultar_lookwell_Cue.Kultar_lookwell_Cue")
      (if (Math|Random|RandomBool) :!label _label
        (Utilities|FlowControl|Delay 2.0)
        (bind _outactors (Actor|GetAllActorsOfClasswithTag "/Game/NPC/GoblinNPC/NPC_Goblin.NPC_Goblin_C" "Goblin_GuardKultar"))
        (if (not (Variables|/Game/MonsterAi_Kit/Monster_NBC.Monster_NBC_C|GetDead (Utilities|Array|Get(acopy) _outactors)))
          (Audio|PlaySoundatLocation "/Game/NPC/KultarNPC/Song/Goblin_guard_shutup/Goblin_guard_shutup_Cue.Goblin_guard_shutup_Cue" (Transformation|GetActorLocation (Utilities|Array|Get(acopy) _outactors)) "0, 0, 0" 1.0 1.0 0.0 0 0 0))))
    (:2
      (CallFunction|SpeakKultar "/Game/NPC/KultarNPC/Song/Kultar_encourage23_Cue.Kultar_encourage23_Cue")
      (goto _label))
    (:3
      (CallFunction|SpeakKultar "/Game/NPC/KultarNPC/Song/letmeOut/Kultar_letmeout_Cue.Kultar_letmeout_Cue"))
    (:4
      (CallFunction|SpeakKultar "/Game/NPC/KultarNPC/Song/thanksAgain/Kultar_thanks_again_Cue.Kultar_thanks_again_Cue"))))

(event EventBPILoadDone
  ;[1 1 1] Save/Load
  (Save/load|LoadDone))

(event Game|Damage|EventAnyDamage
  (params (Damage :type Float%20%28single-precision%29) (DamageType :type Damage%20Type%20Object%20Reference) (InstigatedBy :type Controller%20Object%20Reference) (DamageCauser :type Actor%20Object%20Reference))
  (Default|StatChanged (Variables|Default|GetBP_Stats) Damage "NewEnumerator38" true))

(event EventBPILoadState
  (params (SaveSlot :type S%20Save%20Actor%20Structure))
  ;[1 1 1] Save/Load
  (Save/load|LoadState SaveSlot))

(event EventTick
  (params (DeltaSeconds :type Float%20%28single-precision%29))
  (if (Variables|Default|GetStoryMode)
    (CallFunction|ScenarioEvent)))

(event EventBInteraction
  (CallFunction|SpecScenario)
  (CallFunction|IInteraction))

(fn ConstructionScript
  (Variables|Default|SetLoc (Transformation|GetActorLocation)))

(fn DestroySelf
  (Actor|DestroyActor))

(fn LoadDone
  (if (not (Variables|Default|GetLoaded))
    (return)))

(fn LoadState
  (params (SaveDataAdd :type S%20Save%20Actor%20Structure))
  (Variables|Default|SetLoaded true)
  (Variables|Default|SetDead (.isdead SaveDataAdd))
  (Transformation|SetActorTransform self (.position SaveDataAdd) false true))

(fn SaveState
  (params (Save%20Data%20Add%20Add :type S%20Save%20Actor%20Add%20Structure))
  (return (Utilities|Struct|MakeS_SaveActor (Transformation|GetActorTransform) (Utilities|GetClass self) (Variables|Default|GetDead) false "(BoolArray_2_0C11053C44F85D099D01009D36B474A2=)" self 0 "(Items_4_E2E953BB4A67DC946206EF9D2DA87881=())" 0 0.0)))

(fn BPISaveState
  (return ""))

(event Custom|ScenarioEvent
  (bind _returnvalue (Game|GetPlayerCharacter 0))
  (bind _asbp_rpg_character_main (Utilities|Casting|CastToBP_RPG_CharacterMain _returnvalue))
  (bind _inventorymodule (Variables|/Game/RPGCharacterCreator/Blueprints/BP_RPG_CharacterMain.BP_RPG_CharacterMain_C|GetInventoryModule _asbp_rpg_character_main))
  (bind _baseui (Variables|/Game/RPGCharacterCreator/Blueprints/BP_InventoryModule.BP_InventoryModule_C|GetBaseUi _inventorymodule))
  (Utilities|FlowControl|Sequence
    (:then_0
      (switch int (Variables|Default|GetScenario)
        (:0
          ;[1 1 1] 1
          (Utilities|FlowControl|DoOnce false
            (:Completed
              (Animation|PlayAnimMontage "/Game/NPC/KultarNPC/KultarSitAnim_Montage.KultarSitAnim_Montage" 1.0 "None")
              (Variables|/Script/Engine.CharacterMovementComponent|SetMaxWalkSpeed (Variables|Character|GetCharacterMovement) 0.0))))
        (:1
          ;[1 1 1] 2
          (Utilities|FlowControl|DoOnce false
            (:Completed
              (Utilities|FlowControl|Delay 1.5)
              (Audio|PlaySoundatLocation "/Game/NPC/KultarNPC/Song/Kultar_Hey_Cue.Kultar_Hey_Cue" (Transformation|GetActorLocation) "0, 0, 0" 1.0 1.0 0.0 0 0 0)
              (Animation|StopAnimMontage "/Game/NPC/KultarNPC/KultarSitAnim_Montage.KultarSitAnim_Montage")
              (Animation|PlayAnimMontage "/Game/NPC/KultarNPC/KultarStay_SK_Kultar1_Anim_Montage.KultarStay_SK_Kultar1_Anim_Montage" 1.0 "None")
              (Utilities|FlowControl|Delay 1.33)
              (Animation|StopAnimMontage "/Game/NPC/KultarNPC/KultarStay_SK_Kultar1_Anim_Montage.KultarStay_SK_Kultar1_Anim_Montage")
              (Variables|Default|SetScenario 2)
              (Variables|/Script/Engine.CharacterMovementComponent|SetMaxWalkSpeed (Variables|Character|GetCharacterMovement) 55.0))))
        (:2
          ;[1 1 1] 3
          (Utilities|FlowControl|DoOnce false
            (:Completed
              (Variables|Default|SetWeapointInt 0)
              (AI|AIMoveTo self (Transformation|GetActorLocation (Utilities|Array|Get(acopy) (Variables|Default|GetWeapoints) (Variables|Default|GetWeapointInt))) 0 5.0 false
                (:OnSuccess
                  (Audio|PlaySoundatLocation "/Game/NPC/KultarNPC/Song/Kultar_introduction_Cue.Kultar_introduction_Cue" (Transformation|GetActorLocation) "0, 0, 0" 1.0 1.0 0.0 0 0 0)
                  (Variables|Default|SetScenario 3)
                  (Variables|Default|SetScenario_Talk 1)
                  (Variables|Default|SetKultarTalk true)
                  (Utilities|FlowControl|Delay 3.0))))))
        (:3
          ;[1 1 1] 4
          (if (Variables|Default|GetKultarTalkStartCinematic)
            (Utilities|FlowControl|DoOnce false
              (:Completed
                (Variables|Default|SetKultarTalk false)
                (bind _outactors (Actor|GetAllActorsOfClass "/Script/LevelSequence.LevelSequenceActor"))
                (Sequencer|Player|Play (Variables|/Script/LevelSequence.LevelSequenceActor|GetSequencePlayer (Utilities|Array|Get(acopy) _outactors)) :!class /Script/MovieScene.MovieSceneSequencePlayer)
                (Utilities|FlowControl|Sequence
                  (:then_0
                    (Default|TalkCharacter _asbp_rpg_character_main true false)
                    (Variables|/Game/RPGCharacterCreator/Blueprints/BP_RPG_CharacterMain.BP_RPG_CharacterMain_C|SetTalk _asbp_rpg_character_main true)
                    (Variables|Default|SetKultarTalk true)
                    (Default|HideHud _baseui false)
                    (Utilities|FlowControl|Delay 18.0)
                    (Default|VisibleHud _baseui)
                    (Default|TalkCharacter _asbp_rpg_character_main false true)
                    (Variables|Default|SetScenario 4)
                    (Variables|/Game/RPGCharacterCreator/Blueprints/BP_RPG_CharacterMain.BP_RPG_CharacterMain_C|SetTalk _asbp_rpg_character_main false)
                    (Variables|Default|SetKultarTalkStartCinematic false)
                    (Variables|Default|SetKultarTalk false))
                  (:then_1
                    (bind _outactors_2 (Actor|GetAllActorsOfClasswithTag "/Game/Blueprints/CinematicPlayerPos.CinematicPlayerPos_C" "1"))
                    (Transformation|SetActorTransform (.AsBP%20RPG%20Character%20Main (Utilities|Casting|CastToBP_RPG_CharacterMain (Game|GetPlayerCharacter 0))) (Transformation|GetActorTransform (Utilities|Array|Get(acopy) _outactors_2)))
                    (Pawn|SetControlRotation (Game|GetPlayerController 0) (Transformation|GetActorRotation (Utilities|Array|Get(acopy) _outactors_2)))))))))
        (:4
          ;[1 1 1] 5
          (bind _outactors_3 (Actor|GetAllActorsOfClasswithTag "/Game/NPC/GoblinNPC/NPC_Goblin.NPC_Goblin_C" "Goblin_GuardKultar"))
          (if (Variables|/Game/MonsterAi_Kit/Monster_NBC.Monster_NBC_C|GetDead (Utilities|Array|Get(acopy) _outactors_3))
            (Utilities|FlowControl|DoOnce false
              (:Completed
                (Variables|Default|SetWeapointInt 1)
                (AI|AIMoveTo self (Transformation|GetActorLocation (Utilities|Array|Get(acopy) (Variables|Default|GetWeapoints) (Variables|Default|GetWeapointInt))) 0 1.0 true
                  (:OnSuccess
                    (Variables|Default|SetScenario 5)
                    (Variables|Default|SetScenario_Talk 3)
                    (CallFunction|SpeakKultar "/Game/NPC/KultarNPC/Song/letmeOut/Kultar_letmeout_Cue.Kultar_letmeout_Cue")))))))
        (:5
          (bind _outactors_4 (Actor|GetAllActorsOfClasswithTag "/Game/Blueprints/DOOR/Lever_Child.Lever_Child_C" "Lever_Kultar" :!label _label))
          (if (Variables|/Game/Blueprints/DOOR/Lever.Lever_C|GetMoving (Utilities|Array|Get(acopy) _outactors_4))
            (if (< (Variables|Default|GetScenario) 5)
              (Variables|Default|SetScip? true))
            (Utilities|FlowControl|DoOnce false
              (:Completed
                (Variables|Default|SetScenario 5)
                (Variables|Default|SetScenario_Talk 3)
                (if (Variables|Default|GetScip?)
                  (Animation|StopAnimMontage "/Game/NPC/KultarNPC/KultarSitAnim_Montage.KultarSitAnim_Montage")
                  (Animation|PlayAnimMontage "/Game/NPC/KultarNPC/KultarStay_SK_Kultar1_Anim_Montage.KultarStay_SK_Kultar1_Anim_Montage" 1.0 "None")
                  (Utilities|FlowControl|Delay 1.33)
                  (Animation|StopAnimMontage "/Game/NPC/KultarNPC/KultarStay_SK_Kultar1_Anim_Montage.KultarStay_SK_Kultar1_Anim_Montage")
                  (Variables|/Script/Engine.CharacterMovementComponent|SetMaxWalkSpeed (Variables|Character|GetCharacterMovement) 55.0))
                ;[1 1 1] 6
                (Utilities|FlowControl|Sequence
                  (:then_0
                    (bind _outactors_5 (Actor|GetAllActorsOfClasswithTag "/Game/Blueprints/CinematicPlayerPos.CinematicPlayerPos_C" "2"))
                    (Transformation|SetActorTransform (CallFunction|--GetPlayerCharacter) (Transformation|GetActorTransform (Utilities|Array|Get(acopy) _outactors_5)))
                    (Pawn|SetControlRotation (Game|GetPlayerController 0) (Transformation|GetActorRotation (Utilities|Array|Get(acopy) _outactors_5)))
                    (Default|HideHud (Variables|/Game/RPGCharacterCreator/Blueprints/BP_InventoryModule.BP_InventoryModule_C|GetBaseUi (Variables|/Game/RPGCharacterCreator/Blueprints/BP_RPG_CharacterMain.BP_RPG_CharacterMain_C|GetInventoryModule (CallFunction|--GetPlayerCharacter))) true))
                  (:then_1
                    (bind _outactors_6 (Actor|GetAllActorsOfClass "/Script/LevelSequence.LevelSequenceActor"))
                    (Sequencer|Player|Play (Variables|/Script/LevelSequence.LevelSequenceActor|GetSequencePlayer (Utilities|Array|Get(acopy) _outactors_6 2)) :!class /Script/MovieScene.MovieSceneSequencePlayer)
                    (Variables|/Game/RPGCharacterCreator/Blueprints/BP_RPG_CharacterMain.BP_RPG_CharacterMain_C|SetCinematicON (CallFunction|--GetPlayerCharacter) true)
                    (Variables|Default|SetScenario 6)
                    (Variables|Default|SetWeapointInt 2)
                    (AI|AIMoveTo self (Transformation|GetActorLocation (Utilities|Array|Get(acopy) (Variables|Default|GetWeapoints) (Variables|Default|GetWeapointInt))) 0 0.0 true
                      (:OnSuccess
                        (Variables|Default|SetScenario_Talk 4)
                        (Transformation|SetActorRotation (Transformation|GetActorRotation (Utilities|Array|Get(acopy) (Variables|Default|GetWeapoints) (Variables|Default|GetWeapointInt))))
                        (bind _outactors_7 (Actor|GetAllActorsOfClass "/Script/LevelSequence.LevelSequenceActor"))
                        (Sequencer|Player|Play (Variables|/Script/LevelSequence.LevelSequenceActor|GetSequencePlayer (Utilities|Array|Get(acopy) _outactors_7 1)) :!class /Script/MovieScene.MovieSceneSequencePlayer)
                        (Variables|/Game/RPGCharacterCreator/Blueprints/BP_RPG_CharacterMain.BP_RPG_CharacterMain_C|SetCinematicON (CallFunction|--GetPlayerCharacter) true)
                        (Variables|Default|SetName "Култар")
                        (Utilities|FlowControl|Delay 50.5)
                        (Default|StopCinematics (Variables|Default|GetCinematicViev)))))
                  (:then_2
                    (bind _returnvalue_2 (UserInterface|CreateWidget "/Game/RPGCharacterCreator/UI/CinematicViev.CinematicViev_C"))
                    (bind _output_get (Variables|Default|SetCinematicViev _returnvalue_2))
                    (UserInterface|Viewport|AddtoViewport _output_get 1000)
                    (Default|StartCinematics (Variables|Default|GetCinematicViev))))))))))
    (:then_1
      (goto _label))))

(fn ICanbeInteracted
  (return true))

(fn IEndInteraction
  (params (InteractingCharacter :type Character%20Object%20Reference))
  (return false))

(fn IGetInteractionText
  (return "" ""))

(fn IGetInventoryItems
  (return (Default|GetInventoryItems (Variables|Default|GetBP_InventoryModule))))

(fn IInteraction
  (params (InteractingCharacter :type Character%20Object%20Reference))
  (LocalVariables|SetL_Character InteractingCharacter)
  (if (.IsFound? (CallFunction|GetInventoryComponent (LocalVariables|GetL_Character)))
    (Default|ShowTrade (.Inventory (CallFunction|GetInventoryComponent (LocalVariables|GetL_Character))) self 100)
    (return (Variables|Default|GetName) true)
    (else
      (return (Variables|Default|GetName) true))))

(fn ISetInventoryItems
  (params (Items :type Map%20of%20ST%20Item%20Slot%20Params%20Structures%20to%20Structs))
  (bind _self self)
  (bind (_inventory _isfound_) (CallFunction|GetInventoryComponent _self))
  (if _isfound_
    (Default|SetInventoryItems _inventory Items)
    (return true)
    (else
      (return false))))