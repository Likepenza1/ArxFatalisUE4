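; BP_Anwil is an interactable anvil actor that plays sound when used and remembers whether it has been used.
; Its interaction event triggers a location sound, then UpdateStatus plays the anvil-use sound and sets the used flag on first use only.
; Save/load interface functions persist that flag as the IsOn state.
; The other interaction interface functions are mostly stubs, returning only the Russian anvil name and success.
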(event Custom|Use
  (Utilities|FlowControl|Sequence
    (:then_0
      (Audio|PlaySoundatLocation 0 (Transformation|GetActorLocation) "0, 0, 0" 1.0 1.0 0.0 0 0 0))
    (:then_1
      (CallFunction|UpdateStatus))))

(event EventBInteraction
  (CallFunction|Use))

(event EventBeginPlay)

(event EventBPILoadState
  (params (SaveSlot :type S%20Save%20Actor%20Structure))
  (CallFunction|LoadState SaveSlot))

(event EventBPILoadDone
  (CallFunction|LoadDone))

(fn ConstructionScript)

(fn LoadState
  (params (SaveDataAdd :type S%20Save%20Actor%20Structure))
  (Variables|Default|SetLoaded true)
  (Variables|Default|Set1Used (.ison SaveDataAdd)))

(fn SaveState
  (params (Save%20Data%20Add :type S%20Save%20Actor%20Add%20Structure))
  (return (Utilities|Struct|MakeS_SaveActor "0.000000,0.000000,0.000000|0.000000,0.000000,0.000000|1.000000,1.000000,1.000000" 0 false (Variables|Default|Get1Used) "(BoolArray_2_0C11053C44F85D099D01009D36B474A2=)" 0 0 "(Items_4_E2E953BB4A67DC946206EF9D2DA87881=())" 0 0.0)))

(fn UpdateStatus
  (if (not (Variables|Default|Get1Used))
    (Audio|PlaySoundatLocation "/Game/Meshes/Anwil/player_anvil_use.player_anvil_use" (Transformation|GetActorLocation) "0, 0, 0" 1.0 1.0 0.0 0 0 0)
    (Variables|Default|Set1Used true)))

(fn LoadDone
  (if (not (Variables|Default|GetLoaded))
    (return)))

(fn BPISaveState
  (return (Utilities|Struct|MakeS_SaveActor (Variables|Default|Get1Used))))

(fn ICanbeInteracted
  (return false))

(fn IEndInteraction
  (params (InteractingCharacter :type Character%20Object%20Reference))
  (return false))

(fn IGetInteractionText
  (return "" ""))

(fn IGetInventoryItems
  (return 0))

(fn IInteraction
  (params (InteractingCharacter :type Character%20Object%20Reference))
  (return "Наковальня" true))

(fn ISetInventoryItems
  (params (Items :type Map%20of%20ST%20Item%20Slot%20Params%20Structures%20to%20Structs))
  (return false))