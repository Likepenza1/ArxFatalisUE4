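; Inventory item action that lets the character eat a food item, changing a stat and consuming the item from its slot.
; RunAction passes the item's first stat settings to the inventory component and spawns its use sound, then asks the inventory widget to remove it.
; It reports Handled or Unhandled based on that removal, but calls neither if the initial component or UI check fails.
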(event EventRunAction
  (params (ExecSlot :type WB%201%20Slot%20Container%20Object%20Reference) (Item :type ST%20Character%20Item%20Structure) (ItemSlot :type WB%201%20Slot%20Container%20Object%20Reference))
  (bind (_inventory _isfound_) (CallFunction|GetInventoryComponent))
  (bind (_inventory_2 _isfound__2) (CallFunction|GetInventoryComponent))
  (bind (_valid_ _inventorywidget) (Default|GetBaseUi _inventory))
  (Variables|Default|SetExecSlot ExecSlot)
  (Variables|Default|SetItem Item)
  (Variables|Default|SetItemSlot ItemSlot)
  (if _isfound__2
    (Variables|Default|SetInventoryComponentRef _inventory_2)
    (if (.Valid? (Default|GetBaseUi _inventory_2))
      (Default|-StatsChanged (Variables|Default|GetInventoryComponentRef) (.1_StatValue (Utilities|Struct|BreakST_CharacterItem (Variables|Default|GetItem))) (.1_Stat (Utilities|Struct|BreakST_CharacterItem (Variables|Default|GetItem))) (.1_StatRemoved (Utilities|Struct|BreakST_CharacterItem (Variables|Default|GetItem))))
      (Default|-SpawnSoundUsed (Variables|Default|GetInventoryComponentRef) (.SoundUsed (Utilities|Struct|BreakST_CharacterItem (Variables|Default|GetItem))))
      (if _isfound_
        (if _valid_
          (bind _removed (Default|RemoveItemfromSlot _inventorywidget (Variables|Default|GetItemSlot)))
          (if _removed
            (CallFunction|Handled)
            (else
              (CallFunction|Unhandled :!label _label)))
          (else
            (goto _label)))
        (else
          (goto _label))))))