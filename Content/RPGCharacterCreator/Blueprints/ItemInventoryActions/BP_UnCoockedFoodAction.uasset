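; BP_UnCoockedFoodAction is an inventory item action, named for uncooked food, that runs when an item slot is executed.
; RunAction stores the slot and item data, finds the inventory component, and plays the item's use sound through it if the base UI is valid.
; It then calls Unhandled after an empty component check, applying no food effect of its own.
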(event EventRunAction
  (params (ExecSlot :type WB%201%20Slot%20Container%20Object%20Reference) (Item :type ST%20Character%20Item%20Structure) (ItemSlot :type WB%201%20Slot%20Container%20Object%20Reference))
  (bind (_inventory _isfound_) (CallFunction|GetInventoryComponent))
  (Variables|Default|SetExecSlot ExecSlot)
  (Variables|Default|SetItem Item)
  (Variables|Default|SetItemSlot ItemSlot)
  (if _isfound_
    (Variables|Default|SetInventoryComponentRef _inventory)
    (if (.Valid? (Default|GetBaseUi _inventory))
      (Default|-SpawnSoundUsed (Variables|Default|GetInventoryComponentRef) (Utilities|Struct|BreakST_CharacterItem (Variables|Default|GetItem)))
      (if (.IsFound? (CallFunction|GetInventoryComponent))
        _
        (else
          _))
      (CallFunction|Unhandled))))