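; Inventory action that equips an item when the player meets its four stat requirements, otherwise plays a not-skilled-enough sound.
; An equipment slot container target limits equipping to its compatible slots, while other targets use auto slot detection.
; On success it applies four stat changes, flat or as a percentage of the current stat, and plays the item's sound.
; It reports Handled only after removing the item from its inventory UI slot.
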(event EventRunAction
  (params (ExecSlot :type WB%201%20Slot%20Container%20Object%20Reference) (Item :type ST%20Character%20Item%20Structure) (ItemSlot :type WB%201%20Slot%20Container%20Object%20Reference))
  (bind (_inventory _isfound_) (CallFunction|GetInventoryComponent))
  (bind (_inventory_2 _isfound__2) (CallFunction|GetInventoryComponent))
  (bind (_valid_ _inventorywidget) (Default|GetBaseUi _inventory))
  (Variables|Default|SetExecSlot ExecSlot)
  (Variables|Default|SetItem Item)
  (Variables|Default|SetItemSlot ItemSlot)
  (if _isfound__2
    (Variables|Default|SetInventoryComponentRef _inventory_2)
    (if (CallFunction|IsObjectEmpty (Variables|Default|GetExecSlot) true)
      (if (Math|Boolean|ANDBoolean (>= (Default|-StatChecked (Variables|Default|GetInventoryComponentRef) (.1_NeedStats (Utilities|Struct|BreakST_CharacterItem (Variables|Default|GetItem)))) (.1_Stats_Needed (Utilities|Struct|BreakST_CharacterItem (Variables|Default|GetItem)))) (>= (Default|-StatChecked (Variables|Default|GetInventoryComponentRef) (.2_NeedStats (Utilities|Struct|BreakST_CharacterItem (Variables|Default|GetItem)))) (.2_Stats_Needed (Utilities|Struct|BreakST_CharacterItem (Variables|Default|GetItem)))) (>= (Default|-StatChecked (Variables|Default|GetInventoryComponentRef) (.3_NeedStats (Utilities|Struct|BreakST_CharacterItem (Variables|Default|GetItem)))) (.3_Stats_Needed (Utilities|Struct|BreakST_CharacterItem (Variables|Default|GetItem)))) (>= (Default|-StatChecked (Variables|Default|GetInventoryComponentRef) (.4_NeedStats (Utilities|Struct|BreakST_CharacterItem (Variables|Default|GetItem)))) (.4_Stats_Needed (Utilities|Struct|BreakST_CharacterItem (Variables|Default|GetItem)))))
        ;[1 1 1] Можно ли установить этот предмет именно в этот слот?
        (bind _aswb_equipment_slot_container (Utilities|Casting|CastToWB_EquipmentSlotContainer (Variables|Default|GetExecSlot))
          (:then
            ;[1 1 1] установите предмет в текущий слот
            (for _array_element (Variables|/Game/RPGCharacterCreator/UI/Controls/Inventory/Containers/WB_EquipmentSlotContainer.WB_EquipmentSlotContainer_C|GetEquipmentSlots _aswb_equipment_slot_container)
              (if (Utilities|Array|ContainsItem (Default|GetItemEquipmentSlots (Variables|Default|GetInventoryComponentRef) (Variables|Default|GetItem) false) _array_element)
                (bind _success_ (Default|EquipItemtoSlot (Variables|Default|GetInventoryComponentRef) (Variables|Default|GetItem) true true true _array_element))
                (if _success_
                  (Variables|Default|SetEquipped? true)))))
          (:CastFailed
            ;[1 1 1] Equip Item with auto slot detection
            (bind _success__2 (Default|EquipItem (Variables|Default|GetInventoryComponentRef) (Variables|Default|GetItem) true true true))
            (Variables|Default|SetEquipped? _success__2)))
        (if (Variables|Default|GetEquipped?)
          (Default|-StatsChanged (Variables|Default|GetInventoryComponentRef) (Utilities|Percent (.1_Stat (Utilities|Struct|BreakST_CharacterItem (Variables|Default|GetItem))) (.1_StatValue (Utilities|Struct|BreakST_CharacterItem (Variables|Default|GetItem))) (.1_StatPercent (Utilities|Struct|BreakST_CharacterItem (Variables|Default|GetItem)))) (.1_Stat (Utilities|Struct|BreakST_CharacterItem (Variables|Default|GetItem))) (.1_StatRemoved (Utilities|Struct|BreakST_CharacterItem (Variables|Default|GetItem))))
          (Default|-StatsChanged (Variables|Default|GetInventoryComponentRef) (Utilities|Percent (.2_Stat (Utilities|Struct|BreakST_CharacterItem (Variables|Default|GetItem))) (.2_StatValue (Utilities|Struct|BreakST_CharacterItem (Variables|Default|GetItem))) (.2_StatPercent (Utilities|Struct|BreakST_CharacterItem (Variables|Default|GetItem)))) (.2_Stat (Utilities|Struct|BreakST_CharacterItem (Variables|Default|GetItem))) (.2_StatRemoved (Utilities|Struct|BreakST_CharacterItem (Variables|Default|GetItem))))
          (Default|-StatsChanged (Variables|Default|GetInventoryComponentRef) (Utilities|Percent (.3_Stat (Utilities|Struct|BreakST_CharacterItem (Variables|Default|GetItem))) (.3_StatValue (Utilities|Struct|BreakST_CharacterItem (Variables|Default|GetItem))) (.3_StatPercent (Utilities|Struct|BreakST_CharacterItem (Variables|Default|GetItem)))) (.3_Stat (Utilities|Struct|BreakST_CharacterItem (Variables|Default|GetItem))) (.3_StatRemoved (Utilities|Struct|BreakST_CharacterItem (Variables|Default|GetItem))))
          (Default|-StatsChanged (Variables|Default|GetInventoryComponentRef) (Utilities|Percent (.4_Stat (Utilities|Struct|BreakST_CharacterItem (Variables|Default|GetItem))) (.4_StatValue (Utilities|Struct|BreakST_CharacterItem (Variables|Default|GetItem))) (.4_StatPercent (Utilities|Struct|BreakST_CharacterItem (Variables|Default|GetItem)))) (.4_Stat (Utilities|Struct|BreakST_CharacterItem (Variables|Default|GetItem))) (.4_StatRemoved (Utilities|Struct|BreakST_CharacterItem (Variables|Default|GetItem))))
          (Default|-SpawnSoundUsed (Variables|Default|GetInventoryComponentRef) (.SoundUsed (Utilities|Struct|BreakST_CharacterItem (Variables|Default|GetItem))))
          (if _isfound_
            (if _valid_
              (bind _removed (Default|RemoveItemfromSlot _inventorywidget (Variables|Default|GetItemSlot)))
              (if _removed
                (CallFunction|Handled)
                (else
                  (CallFunction|Unhandled :!label _label)))
              (else
                (goto _label)))
            (else
              (goto _label)))
          (else
            (goto _label)))
        (else
          (Default|-SpawnSoundUsed (Variables|Default|GetInventoryComponentRef) "/Game/player_not_skilled_enough.player_not_skilled_enough")
          (CallFunction|Unhandled))))))