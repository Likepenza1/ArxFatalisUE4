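; BP_Stats holds RPG character stats as an array of base, modifier and max values, firing events when base values or modifiers change.
; StatChanged raises or lowers base values, clamping overflow at zero or max.
; Atribut functions, including Razum (Intellect) and Lovkost (Agility) variants, propagate attribute changes into other stats via fixed amounts, level-indexed tables or modulo intervals.
; GetDamage applies a chance-based, crit-style multiplier, ignoring modifiers.
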(fn RemoveModifier
  (params (Type :type E_PlayerStats%20Enum :default "NewEnumerator0") (Value :type Integer))
  (if (!= Value 0)
    (bind _output_get (LocalVariables|SetL_Index (Stats|GetStatIndex Type)))
    (if (>= _output_get 0)
      (Utilities|Struct|SetmembersinS_Stat (Utilities|Array|Get(acopy) (Variables|Default|GetStat) (LocalVariables|GetL_Index)) (- (.ModifiersValue (Utilities|Struct|BreakS_Stat (Utilities|Array|Get(acopy) (Variables|Default|GetStat) (LocalVariables|GetL_Index)))) Value))
      (Default|CallOnModifierRemoved Type Value))))

(fn AddModifier
  (params (Type :type E_PlayerStats%20Enum :default "NewEnumerator0") (Value :type Integer))
  (if (!= Value 0)
    (bind _output_get (LocalVariables|SetL_Index (Stats|GetStatIndex Type)))
    (if (>= _output_get 0)
      (Utilities|Struct|SetmembersinS_Stat (Utilities|Array|Get(acopy) (Variables|Default|GetStat) (LocalVariables|GetL_Index)) (+ (.ModifiersValue (Utilities|Struct|BreakS_Stat (Utilities|Array|Get(acopy) (Variables|Default|GetStat) (LocalVariables|GetL_Index)))) Value))
      (Default|CallOnModifierAdded Type Value))))

(fn ChangeStatBaseValue
  (params (Type :type E_PlayerStats%20Enum :default "NewEnumerator0") (NewValue :type Integer))
  (Utilities|Struct|SetmembersinS_Stat (Utilities|Array|Get(acopy) (Variables|Default|GetStat) (Stats|GetStatIndex Type)) NewValue)
  (Default|CallOnBaseValueChanged Type NewValue))

(fn GetDamage
  (return (* (.Value (Stats|GetStatValue "NewEnumerator4" false)) (select (<= (Math|Random|RandomIntegerinRange 1 100) (.Value (Stats|GetStatValue "NewEnumerator0" false))) (.Value (Stats|GetStatValue "NewEnumerator15" false)) 1))))

(fn GetStatIndex
  (params (PlayerStats :type E_PlayerStats%20Enum :default "NewEnumerator0"))
  (for (_array_element _array_index) (Variables|Default|GetStat)
    (if (Utilities|Enum|Equal(Enum) (Utilities|Struct|BreakS_Stat _array_element) PlayerStats)
      (return _array_index)))
  (return -1))

(fn GetStatValue
  (params (PlayerStats :type E_PlayerStats%20Enum :default "NewEnumerator0") (IncludeModifiers :type Boolean))
  (bind _output_get (LocalVariables|SetL_Index (Stats|GetStatIndex PlayerStats)))
  (if (>= _output_get 0)
    (return (Math|Integer|SelectInt (.BaseValue (Utilities|Struct|BreakS_Stat (Utilities|Array|Get(acopy) (Variables|Default|GetStat) (LocalVariables|GetL_Index)))) (+ (.BaseValue (Utilities|Struct|BreakS_Stat (Utilities|Array|Get(acopy) (Variables|Default|GetStat) (LocalVariables|GetL_Index)))) (.ModifiersValue (Utilities|Struct|BreakS_Stat (Utilities|Array|Get(acopy) (Variables|Default|GetStat) (LocalVariables|GetL_Index))))) IncludeModifiers) (.MaxValue (Utilities|Struct|BreakS_Stat (Utilities|Array|Get(acopy) (Variables|Default|GetStat) (LocalVariables|GetL_Index)))))))

(fn StatChanged
  (params (Value :type Integer) (Type :type E_PlayerStats%20Enum :default "NewEnumerator0") (Removed? :type Boolean))
  (bind (_value _maxvalue) (Stats|GetStatValue Type false))
  (bind _returnvalue (- _value Value))
  (bind _returnvalue_2 (+ Value _value))
  (LocalVariables|SetL_MaxValue _maxvalue)
  (LocalVariables|SetL_Value _value)
  (if (!= Value 0)
    (if (>= _value 0)
      (if Removed?
        (Stats|ChangeStatBaseValue Type _returnvalue)
        (if (<= _returnvalue 0)
          (Stats|ChangeStatBaseValue Type)
          ;[1 1 1] -
          (Default|CallOnTakeDamage Value))
        (else
          (Stats|ChangeStatBaseValue Type _returnvalue_2)
          (if (>= _returnvalue_2 (LocalVariables|GetL_MaxValue))
            (Stats|ChangeStatBaseValue Type (LocalVariables|GetL_MaxValue))
            ;[1 1 1] +
            (Default|CallOnTakeDamage Value)))))))

(fn Atribut
  (params (Removed? :type Boolean) (Attribut :type E_PlayerStats%20Enum :default "NewEnumerator0") (ChangeParam-1 :type E_PlayerStats%20Enum :default "NewEnumerator0") (ChangeParam-1%20Value :type Integer) (Param-1%20Interval :type Integer) (1--- :type Boolean) (ChangeParam-2 :type E_PlayerStats%20Enum :default "NewEnumerator0") (ChangeParam-2%20Value :type Integer) (Param-2%20Interval :type Integer) (2--- :type Boolean) (ChangeParam-3 :type E_PlayerStats%20Enum :default "NewEnumerator0") (ChangeParam-3%20Value :type Integer) (Param-3%20Interval :type Integer) (3--- :type Boolean) (ChangeParam-4 :type E_PlayerStats%20Enum :default "NewEnumerator0") (ChangeParam-4%20Value :type Integer) (Param-4%20Interval :type Integer) (4--- :type Boolean) (ChangeParam-5 :type E_PlayerStats%20Enum :default "NewEnumerator0") (ChangeParam-5%20Value :type Integer) (Param-5%20Interval :type Integer))
  (CallFunction|StatChanged ChangeParam-1%20Value ChangeParam-1 Removed?)
  (CallFunction|StatChanged ChangeParam-2%20Value ChangeParam-2 Removed?)
  (CallFunction|StatChanged ChangeParam-3%20Value ChangeParam-3 Removed?)
  (CallFunction|StatChanged ChangeParam-4%20Value ChangeParam-4 Removed?)
  (if (== (Math|Integer|%(Integer) (.Value (Stats|GetStatValue Attribut false)) Param-5%20Interval) 0)
    (CallFunction|StatChanged ChangeParam-5%20Value ChangeParam-5 Removed?)
    (else
      (return))))

(fn AtributRazum
  (params (Removed? :type Boolean) (Attribut :type E_PlayerStats%20Enum :default "NewEnumerator0") (ChangeParam-1 :type E_PlayerStats%20Enum :default "NewEnumerator0") (String%201%20param :type Array%20of%20Strings) (ChangeParam-2 :type E_PlayerStats%20Enum :default "NewEnumerator0") (ChangeParam-2%20Value :type Integer) (ChangeParam-3 :type E_PlayerStats%20Enum :default "NewEnumerator0") (ChangeParam-3%20Value :type Integer) (ChangeParam-4 :type E_PlayerStats%20Enum :default "NewEnumerator0") (ChangeParam-4%20Value :type Integer) (ChangeParam-5 :type E_PlayerStats%20Enum :default "NewEnumerator0") (ChangeParam-5%20Value :type Integer) (ChangeParam-6 :type E_PlayerStats%20Enum :default "NewEnumerator0") (String%206%20param :type Array%20of%20Strings) (ChangeParam-7 :type E_PlayerStats%20Enum :default "NewEnumerator0") (ChangeParam-7%20Value :type Integer) (Character%20lvl :type Integer))
  (CallFunction|StatChanged (Math|Conversions|ToInteger(Byte) (Utilities|Array|Get(acopy) String%201%20param (.Value (Stats|GetStatValue Attribut false)))) ChangeParam-1 Removed?)
  (CallFunction|StatChanged ChangeParam-2%20Value ChangeParam-2 Removed?)
  (CallFunction|StatChanged ChangeParam-3%20Value ChangeParam-3 Removed?)
  (CallFunction|StatChanged ChangeParam-4%20Value ChangeParam-4 Removed?)
  (CallFunction|StatChanged ChangeParam-5%20Value ChangeParam-5 Removed?)
  (CallFunction|StatChanged (Math|Conversions|ToInteger(Byte) (Utilities|Array|Get(acopy) String%206%20param (.Value (Stats|GetStatValue Attribut false)))) ChangeParam-6 Removed?)
  (CallFunction|StatChanged ChangeParam-7%20Value ChangeParam-7 Removed?))

(fn AtributLovkost
  (params (Removed? :type Boolean) (Attribut :type E_PlayerStats%20Enum :default "NewEnumerator0") (ChangeParam-1 :type E_PlayerStats%20Enum :default "NewEnumerator0") (ChangeParam-1%20Value :type Integer) (ChangeParam-2 :type E_PlayerStats%20Enum :default "NewEnumerator0") (ChangeParam-2%20Value :type Integer) (ChangeParam-3 :type E_PlayerStats%20Enum :default "NewEnumerator0") (String%203%20param :type Array%20of%20Strings) (ChangeParam-4 :type E_PlayerStats%20Enum :default "NewEnumerator0") (ChangeParam-4%20Value :type Integer) (ChangeParam-5 :type E_PlayerStats%20Enum :default "NewEnumerator0") (ChangeParam-5%20Value :type Integer) (ChangeParam-6 :type E_PlayerStats%20Enum :default "NewEnumerator0") (String%206%20param :type Array%20of%20Strings) (Character%20lvl :type Integer))
  (CallFunction|StatChanged ChangeParam-1%20Value ChangeParam-1 Removed?)
  (CallFunction|StatChanged ChangeParam-2%20Value ChangeParam-2 Removed?)
  (CallFunction|StatChanged (Math|Conversions|ToInteger(Byte) (Utilities|Array|Get(acopy) String%203%20param (.Value (Stats|GetStatValue Attribut false)))) ChangeParam-3 Removed?)
  (CallFunction|StatChanged ChangeParam-4%20Value ChangeParam-4 Removed?)
  (CallFunction|StatChanged ChangeParam-5%20Value ChangeParam-5 Removed?)
  (CallFunction|StatChanged (Math|Conversions|ToInteger(Byte) (Utilities|Array|Get(acopy) String%206%20param (.Value (Stats|GetStatValue Attribut false)))) ChangeParam-6 Removed?))

(fn AtributOptional
  (params (Removed? :type Boolean) (OptionalAtribut :type Boolean) (Attribut :type E_PlayerStats%20Enum :default "NewEnumerator0") (ChangeParam-1 :type E_PlayerStats%20Enum :default "NewEnumerator0") (Param%201%20value :type Integer) (Param%201%20interval :type Integer) (ChangeParam-2 :type E_PlayerStats%20Enum :default "NewEnumerator0") (Param%202%20value :type Integer) (Param%202%20interval :type Integer) (ChangeParam-3 :type E_PlayerStats%20Enum :default "NewEnumerator0") (Param%203%20value :type Integer) (Param%203%20interval :type Integer))
  (if OptionalAtribut
    (if (== (Math|Integer|%(Integer) (.Value (Stats|GetStatValue Attribut false)) Param%201%20interval) 0)
      (CallFunction|StatChanged Param%201%20value ChangeParam-1 Removed?)
      (elif (== (Math|Integer|%(Integer) (.Value (Stats|GetStatValue Attribut false)) Param%202%20interval) 0)
        (CallFunction|StatChanged Param%202%20value ChangeParam-2 Removed?)
        (elif (== (Math|Integer|%(Integer) (.Value (Stats|GetStatValue Attribut false)) Param%203%20interval) 0)
          (CallFunction|StatChanged Param%203%20value ChangeParam-3 Removed?)
          (else
            (return)))))
    (else
      (return))))