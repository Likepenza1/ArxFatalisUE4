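; BP_RPG_CharacterTrade is a trader NPC character whose shop opens when another character interacts with it.
; It implements the interaction functions and always reports itself as interactable.
; On interaction it finds the interacting character's inventory component and calls ShowTrade on it, passing itself and its SellPriceCharge.
; The event graph holds no active logic.
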(event EventBeginPlay
  (|CallParentFunction) ; This node is disabled and will not be called.\nDrag off pins to build functionality.
)

(event Collision|EventActorBeginOverlap
  (params (OtherActor :type Actor%20Object%20Reference)))

(event EventTick
  (params (DeltaSeconds :type Float%20%28single-precision%29)))

(fn ConstructionScript
  (|CallParentFunction))

(fn ICanbeInteracted
  ;[1 1 1] This is Trade NPC so we can see it's shop
  (return true))

(fn IInteraction
  (params (InteractingCharacter :type Character%20Object%20Reference))
  (LocalVariables|SetLInteractionCharacter InteractingCharacter)
  (if (.IsFound? (CallFunction|GetInventoryComponent (LocalVariables|GetLInteractionCharacter)))
    (Default|ShowTrade (.Inventory (CallFunction|GetInventoryComponent (LocalVariables|GetLInteractionCharacter))) self (Variables|Default|GetSellPriceCharge))
    (return true "")))