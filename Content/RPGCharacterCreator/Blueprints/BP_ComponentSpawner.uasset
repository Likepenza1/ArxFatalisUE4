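; BP_ComponentSpawner is a helper Blueprint in the RPG Character Creator that adds components to a given character at runtime.
; It has one function per type: skeletal mesh, static mesh, sphere, box and capsule collision, and spring arm.
; Each wraps the matching Add Component node on the passed Character, forwards manual attachment and relative transform, and returns the new component.
; It holds no other logic, as its event graph and construction script are empty.
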(event EventBeginPlay)

(event Collision|EventActorBeginOverlap
  (params (OtherActor :type Actor%20Object%20Reference)))

(event EventTick
  (params (DeltaSeconds :type Float%20%28single-precision%29)))

(fn ConstructionScript)

(fn SpawnSkeletalMeshComponent
  (params (Character :type Character%20Object%20Reference) (bManualAttachment :type Boolean) (RelativeTransform :type Transform))
  (bind _returnvalue (AddComponent|AddSkeletalMeshComponent Character bManualAttachment RelativeTransform))
  (return _returnvalue))

(fn SpawnStaticMeshComponent
  (params (Character :type Character%20Object%20Reference) (bManualAttachment :type Boolean) (RelativeTransform :type Transform))
  (bind _returnvalue (AddComponent|AddStaticMeshComponent Character bManualAttachment RelativeTransform))
  (return _returnvalue))

(fn SpawnSphereCollisionComponent
  (params (Character :type Character%20Object%20Reference) (bManualAttachment :type Boolean) (RelativeTransform :type Transform))
  (bind _returnvalue (AddComponent|AddSphereComponent Character bManualAttachment RelativeTransform))
  (return _returnvalue))

(fn SpawnBoxCollisionComponent
  (params (Character :type Character%20Object%20Reference) (bManualAttachment :type Boolean) (RelativeTransform :type Transform))
  (bind _returnvalue (AddComponent|AddBoxComponent Character bManualAttachment RelativeTransform))
  (return _returnvalue))

(fn SpawnCapsuleCollisionComponent
  (params (Character :type Character%20Object%20Reference) (bManualAttachment :type Boolean) (RelativeTransform :type Transform))
  (bind _returnvalue (AddComponent|AddCapsuleComponent Character bManualAttachment RelativeTransform))
  (return _returnvalue))

(fn SpawnSpringArmComponent
  (params (Character :type Character%20Object%20Reference) (bManualAttachment :type Boolean) (RelativeTransform :type Transform))
  (bind _returnvalue (AddComponent|AddSpringArmComponent Character bManualAttachment RelativeTransform))
  (return _returnvalue))