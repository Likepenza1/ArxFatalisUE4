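; Base Blueprint for inventory item actions in the RPG character creator, meant for child Blueprints to override RunAction with custom behavior.
; Begin stores the owning character and clears a handled flag, which the default RunAction sets and IsHandled reports.
; Helper functions find components on the owner, chaining from BP_InventoryModule to its inventory widget and any slot being dragged, with validity flags along the way.
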(event Custom|RunAction
  (params (ExecSlot :type WB%201%20Slot%20Container%20Object%20Reference) (Item :type ST%20Character%20Item%20Structure) (ItemSlot :type WB%201%20Slot%20Container%20Object%20Reference))
  ;[0 0.183 1] Override this function in ChildBlueprints to create custom action callbacks
  (Result|Handled))

(event Custom|Begin
  (params (Owner :type Character%20Object%20Reference))
  (Variables|Default|SetOwningCharacter Owner)
  (Result|Unhandled))

(fn GetComponent
  (params (ComponentClass :type Actor%20Component%20Class%20Reference))
  (bind _owningcharacter (Variables|Default|GetOwningCharacter))
  (bind _returnvalue (Actor|GetComponentbyClass _owningcharacter ComponentClass))
  (if (CallFunction|IsObjectEmpty _returnvalue true)
    (return _returnvalue true)
    (else
      (return 0 false))))

(fn GetInventoryComponent
  (bind (_actorcomponent _isfound_) (CallFunction|GetComponent "/Game/RPGCharacterCreator/Blueprints/BP_InventoryModule.BP_InventoryModule_C"))
  (if _isfound_
    (bind _asinventory_module (Utilities|Casting|CastToBP_InventoryModule _actorcomponent)
      (:then
        (return _asinventory_module true))
      (:CastFailed
        _)))
  (return 0 false))

(fn IsObjectEmpty
  (params (Object :type Object%20Object%20Reference) (Not :type Boolean))
  (bind _returnvalue (Utilities|GetObjectName Object))
  (bind _returnvalue_2 (Utilities|Enum|Equal(Enum) _returnvalue "None"))
  (if Not
    (return (not _returnvalue_2))
    (else
      (return _returnvalue_2))))

(fn GetInventoryUi
  (bind (_inventory _isfound_) (CallFunction|GetInventoryComponent))
  (bind (_valid_ _inventorywidget) (Default|GetBaseUi _inventory))
  (if _isfound_
    (return _valid_ _inventorywidget)
    (else
      (return false 0))))

(fn Handled
  (Variables|Result|SetHandleState true))

(fn Unhandled
  (Variables|Result|SetHandleState false))

(fn IsHandled?
  (return (Variables|Result|GetHandleState)))

(fn GetDragandDropWidget
  (bind (_valid_ _inventorywidget) (CallFunction|GetInventoryUi))
  (bind (_yes _dragslotwidget) (Default|SlotDragged? _inventorywidget))
  (if _valid_
    (return _yes _dragslotwidget)))