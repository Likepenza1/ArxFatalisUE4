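; Anim notify state, shown as Player_Collisions, that marks the weapon hit window in RPG character attack animations.
; On begin it sets AttackRelease on BP_RPG_CharacterMain and runs one short Visibility line trace forward from the follow camera, passing the result to LineTraceWeaponColisions.
; The trace follows the camera rather than the weapon and is not repeated during the window.
; On end it clears AttackRelease and Hit.
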(fn GetNotifyName
  (return "Player_Collisions"))

(fn ReceivedNotifyBegin
  (params (MeshComp :type Skeletal%20Mesh%20Component%20Object%20Reference) (Animation :type Anim%20Sequence%20Base%20Object%20Reference) (TotalDuration :type Float%20%28single-precision%29))
  (bind _asbp_rpg_character_main (Utilities|Casting|CastToBP_RPG_CharacterMain (Components|GetOwner MeshComp)))
  (Variables|/Game/RPGCharacterCreator/Blueprints/BP_RPG_CharacterMain.BP_RPG_CharacterMain_C|SetAttackRelease? _asbp_rpg_character_main true)
  (bind (_outhit _returnvalue) (Collision|LineTraceByChannel _asbp_rpg_character_main (Transformation|GetWorldLocation (Variables|/Game/RPGCharacterCreator/Blueprints/BP_RPG_CharacterMain.BP_RPG_CharacterMain_C|GetFollowCamera _asbp_rpg_character_main)) (+ (Transformation|GetWorldLocation (Variables|/Game/RPGCharacterCreator/Blueprints/BP_RPG_CharacterMain.BP_RPG_CharacterMain_C|GetFollowCamera _asbp_rpg_character_main)) (* (Math|Vector|GetForwardVector (Variables|/Game/RPGCharacterCreator/Blueprints/BP_RPG_CharacterMain.BP_RPG_CharacterMain_C|GetFollowCamera _asbp_rpg_character_main)) 1.5e+02)) "TraceTypeQuery1" false 0 "None"))
  (Default|LineTraceWeaponColisions _asbp_rpg_character_main _returnvalue _outhit)
  (return true))

(fn ReceivedNotifyEnd
  (params (MeshComp :type Skeletal%20Mesh%20Component%20Object%20Reference) (Animation :type Anim%20Sequence%20Base%20Object%20Reference))
  (bind _asbp_rpg_character_main (Utilities|Casting|CastToBP_RPG_CharacterMain (Components|GetOwner MeshComp)))
  (Variables|/Game/RPGCharacterCreator/Blueprints/BP_RPG_CharacterMain.BP_RPG_CharacterMain_C|SetAttackRelease? _asbp_rpg_character_main false)
  (Variables|/Game/RPGCharacterCreator/Blueprints/BP_RPG_CharacterMain.BP_RPG_CharacterMain_C|SetHit _asbp_rpg_character_main false)
  (return false))