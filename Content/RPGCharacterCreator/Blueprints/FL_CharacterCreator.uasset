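; FL_CharacterCreator is a shared function library of general-purpose helpers for the RPG character creator.
; It covers sphere and line traces, component, camera and floor lookups, ragdoll toggling, interaction checks and custom cursor setup.
; Small utilities handle empty checks, string and number cleanup, mesh and material slot names, and inventory item stacks and quality colors.
; Many functions build on IsObjectEmpty and GetComponent to return safe fallbacks for missing objects.
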(fn TraceObjectsAroundCharacter
  (params (Actor :type Actor%20Object%20Reference) (Radius :type Float%20%28single-precision%29) (DrawDebugType :type EDrawDebugTrace%20Enum :default "None") (bIgnoreSelf :type Boolean))
  (bind _returnvalue (Transformation|GetActorLocation Actor))
  (bind (_outhits _returnvalue_2) (Collision|MultiSphereTraceForObjects Actor _returnvalue (* _returnvalue "100.000000,100.000000,100.000000") Radius (Utilities|Array|MakeArray "ObjectTypeQuery1" "ObjectTypeQuery2" "ObjectTypeQuery3" "ObjectTypeQuery4" "ObjectTypeQuery6" "ObjectTypeQuery5") false 0 DrawDebugType bIgnoreSelf))
  (if _returnvalue_2
    (Utilities|Array|Clear (LocalVariables|GetMultisphereTraceHitObject))
    (Utilities|Array|Clear (LocalVariables|GetMultisphereTraceTransform))
    (for _array_element _outhits
      (if (Physics|IsSimulatingPhysics (.hitcomponent _array_element) "None")
        (Utilities|Array|Add (LocalVariables|GetMultisphereTraceHitObject) (.hitcomponent _array_element))
        (Utilities|Array|Add (LocalVariables|GetMultisphereTraceTransform) (Transformation|GetWorldTransform (.hitcomponent _array_element)))))
    (return (LocalVariables|GetMultisphereTraceHitObject) (LocalVariables|GetMultisphereTraceTransform) (Transformation|GetActorTransform Actor))))

(fn RemovePrefix
  (params (String%20With%20Prefix :type String) (bSearchFromEnd :type Boolean))
  (bind _returnvalue (Utilities|String|Len String%20With%20Prefix))
  (bind _delimiter (LocalVariables|GetDelimiter))
  (bind _returnvalue_2 (Utilities|String|FindSubstring String%20With%20Prefix _delimiter false bSearchFromEnd))
  (bind _returnvalue_3 (Utilities|String|Len _delimiter))
  (bind _returnvalue_4 (+ _returnvalue_2 _returnvalue_3))
  (if (<= _returnvalue_4 _returnvalue)
    (return (Utilities|String|GetSubstring String%20With%20Prefix _returnvalue_4 _returnvalue))
    (else
      (return String%20With%20Prefix))))

(fn AddPrefix
  (params (OriginalString :type String) (Prefix :type String))
  (return (Utilities|String|Append Prefix (LocalVariables|GetDelimiter) OriginalString)))

(fn HasSubstring
  (params (String :type String) (Substring :type String))
  (return (>= (Utilities|String|FindSubstring String Substring) 0)))

(fn LoadCustomMouseCursor
  (params (CursorSize :type Float%20%28single-precision%29) (Player%20Controller :type Player%20Controller%20Object%20Reference))
  (LocalVariables|SetLCursorSize CursorSize)
  (LocalVariables|SetLPlayerController Player%20Controller)
  (Variables|/Script/Engine.PlayerController|SetbEnableClickEvents Player%20Controller true)
  (Variables|/Script/Engine.PlayerController|SetbEnableMouseOverEvents Player%20Controller true)
  (Variables|/Script/Engine.PlayerController|SetbEnableTouchEvents Player%20Controller true)
  (Variables|/Script/Engine.PlayerController|SetCurrentMouseCursor Player%20Controller "Default")
  (Utilities|FlowControl|Sequence
    (:then_0
      ;[1 1 1] Default Cursor
      (bind _returnvalue (UserInterface|CreateWidget "/Game/RPGCharacterCreator/UI/cursor/CursorDefault.CursorDefault_C" (LocalVariables|GetLPlayerController)))
      (Class|PlayerController|SetMouseCursorWidget (LocalVariables|GetLPlayerController) "Default" _returnvalue))
    (:then_1
      ;[1 1 1] for different cursor types you can make different widgets with images. To change current cursor type do: get player controller -> set current mouse cursor
      (bind _returnvalue_2 (UserInterface|CreateWidget "/Game/RPGCharacterCreator/UI/cursor/CursorDefault.CursorDefault_C" (LocalVariables|GetLPlayerController)))
      (Class|PlayerController|SetMouseCursorWidget (LocalVariables|GetLPlayerController) "GrabHand" _returnvalue_2))))

(fn LineTracefromCursor
  (params (PlayerControler :type Player%20Controller%20Object%20Reference) (DrawDebugType :type EDrawDebugTrace%20Enum :default "None") (LineTraceLength :type Integer))
  (bind (_worldlocation _worlddirection _returnvalue) (Game|Player|ConvertMouseLocationToWorldSpace PlayerControler))
  (if _returnvalue
    (bind (_outhit _returnvalue_2) (Collision|LineTraceByChannel PlayerControler _worldlocation (+ _worldlocation (* _worlddirection LineTraceLength)) "TraceTypeQuery1" false (Utilities|Array|MakeArray PlayerControler) DrawDebugType))
    (return _returnvalue_2 _outhit)
    (else
      (return false ""))))

(fn LineTracefromCamera
  (params (PlayerCharacter :type Character%20Object%20Reference) (DrawDebugType :type EDrawDebugTrace%20Enum :default "None") (LineTraceLength :type Integer) (TraceChannel :type ETraceTypeQuery%20Enum :default "TraceTypeQuery2"))
  (bind _returnvalue (Actor|GetComponentbyClass PlayerCharacter "/Script/Engine.CameraComponent"))
  (bind _returnvalue_2 (Transformation|GetWorldLocation _returnvalue))
  (if (Object|IsObjectEmpty PlayerCharacter true)
    (if (Object|IsObjectEmpty _returnvalue true)
      (bind (_outhit _returnvalue_3) (Collision|LineTraceByChannel PlayerCharacter _returnvalue_2 (+ _returnvalue_2 (* (Math|Vector|GetForwardVector (Transformation|GetWorldRotation _returnvalue)) LineTraceLength)) TraceChannel false (LocalVariables|GetEmptyActorsArray) DrawDebugType))
      (return _returnvalue_3 _outhit)
      (else
        _)))
  (return false ""))

(fn IsObjectEmpty
  (params (Object :type Object%20Object%20Reference) (Not :type Boolean))
  (bind _returnvalue (Utilities|GetObjectName Object))
  (bind _returnvalue_2 (Utilities|IsValid Object))
  (bind _returnvalue_3 (Utilities|Enum|Equal(Enum) _returnvalue "None"))
  (bind _returnvalue_4 (not _returnvalue_2))
  (bind _returnvalue_5 (or _returnvalue_3 _returnvalue_4))
  (if Not
    (return (not _returnvalue_5))
    (else
      (return _returnvalue_5))))

(fn StringEmpty
  (params (String :type String) (Not :type Boolean))
  (bind _returnvalue (Utilities|Enum|Equal(Enum) String "None"))
  (bind _returnvalue_2 (Utilities|Enum|Equal(Enum) String ""))
  (bind _returnvalue_3 (or _returnvalue_2 _returnvalue))
  (if Not
    (return (not _returnvalue_3))
    (else
      (return _returnvalue_3))))

(fn GetInventoryComponent
  (params (ActorOwner :type Actor%20Object%20Reference))
  (bind (_actorcomponent _isfound_) (Component|GetComponent ActorOwner "/Game/RPGCharacterCreator/Blueprints/BP_InventoryModule.BP_InventoryModule_C" ActorOwner))
  (if _isfound_
    (bind _asinventory_module (Utilities|Casting|CastToBP_InventoryModule _actorcomponent)
      (:then
        (return _asinventory_module true))
      (:CastFailed
        _)))
  (return 0 false))

(fn GetComponent
  (params (ActorOwner :type Actor%20Object%20Reference) (ComponentClass :type Actor%20Component%20Class%20Reference))
  (if (Object|IsObjectEmpty ActorOwner true)
    (return (Actor|GetComponentbyClass ActorOwner ComponentClass) true)
    (else
      (return 0 false))))

(fn ModulateFloat
  (params (Nimber :type Float%20%28single-precision%29))
  (if (< Nimber 0.0)
    (return (* Nimber -1.0))
    (else
      (return Nimber))))

(fn CeilVector2D
  (params (Vector2D :type Vector%202D%20Structure))
  (bind (_x _y) (Math|Vector2D|BreakVector2D Vector2D))
  (return (Math|Float|Ceil _x) (Math|Float|Ceil _y)))

(fn If0Then1
  (params (Input :type Integer))
  (if (== Input 0)
    (return 1)
    (else
      (return Input))))

(fn IfMinusThen0
  (params (Number :type Integer))
  (if (< Number 0)
    (return 1)
    (else
      (return Number))))

(fn GetEmptyObject
  (return (LocalVariables|GetObj)))

(fn Rand
  (return (Math|Random|RandomIntegerinRange 0 10000)))

(fn GetSID
  (bind _returnvalue (Game|GetPlayerCharacter 0))
  (bind (_inventory _isfound_) (Component|GetInventoryComponent _returnvalue))
  (if (Object|IsObjectEmpty _returnvalue true)
    (if _isfound_
      (return (+ (+ (Utilities|Map|Length (Variables|/Game/RPGCharacterCreator/Blueprints/BP_InventoryModule.BP_InventoryModule_C|GetInventory _inventory)) (Math|Rand)) (Math|Rand)))
      (else
        (return (Math|Rand))))
    (else
      (return (+ (Math|Rand) (Math|Rand))))))

(fn GetTint
  (params (Color%20Use%20Rule :type ESlateColorStylingMode%20Enum :default "UseColor_Specified"))
  (return (Utilities|Struct|MakeSlateColor "(R=1.000000,G=1.000000,B=1.000000,A=1.000000)" Color%20Use%20Rule) (Utilities|Struct|MakeSlateColor "(R=0.000000,G=0.256678,B=1.000000,A=1.000000)" Color%20Use%20Rule) (Utilities|Struct|MakeSlateColor "(R=1.000000,G=0.000000,B=0.003922,A=1.000000)" Color%20Use%20Rule) (Utilities|Struct|MakeSlateColor "(R=0.074510,G=0.074510,B=0.074510,A=1.000000)" Color%20Use%20Rule) (Utilities|Struct|MakeSlateColor "(R=0.000000,G=0.047059,B=1.000000,A=1.000000)" Color%20Use%20Rule) (Utilities|Struct|MakeSlateColor "(R=1.000000,G=0.000000,B=0.019608,A=1.000000)" Color%20Use%20Rule) (Utilities|Struct|MakeSlateColor "(R=0.164706,G=0.000000,B=0.031373,A=1.000000)" Color%20Use%20Rule)))

(fn MaxIntinArray
  (params (Array :type Array%20of%20Integers))
  (for (_array_element _array_index) Array
    (if (> _array_element (LocalVariables|GetLMax))
      (LocalVariables|SetLMax _array_element)
      (LocalVariables|SetIndex _array_index)))
  (return (LocalVariables|GetLMax) (LocalVariables|GetIndex)))

(fn FormIntfromRange
  (params (Int :type Integer) (Bottom :type Integer) (Top :type Integer))
  (LocalVariables|SetLcInt Int)
  (LocalVariables|SetLcBottom Bottom)
  (LocalVariables|SetLcTop Top)
  (Utilities|FlowControl|Sequence
    (:then_0
      ;[1 1 1] Top
      (if (> (LocalVariables|GetLcInt) (LocalVariables|GetLcTop))
        (return (LocalVariables|GetLcTop))))
    (:then_1
      ;[1 1 1] Bottom
      (if (< (LocalVariables|GetLcInt) (LocalVariables|GetLcBottom))
        (return (LocalVariables|GetLcBottom))))
    (:then_2
      (return (LocalVariables|GetLcInt)))))

(fn IfMinusThenPlusFloat
  (params (Number :type Float%20%28single-precision%29))
  (if (> Number 0.0)
    (return Number)
    (else
      (return (* Number -1.0)))))

(fn IfMinusThenPlusInt
  (params (Number :type Integer))
  (if (>= Number 0)
    (return Number)
    (else
      (return (* Number -1)))))

(fn EnableRagdoll
  (params (Character :type Character%20Object%20Reference))
  (bind _mesh (Variables|/Script/Engine.Character|GetMesh Character))
  (Collision|SetCollisionEnabled (Variables|/Script/Engine.Character|GetCapsuleComponent Character) "NoCollision")
  (Collision|SetCollisionProfileName _mesh "Ragdoll" true :!class /Script/Engine.PrimitiveComponent)
  (Class|SkeletalMeshComponent|SetAllBodiesBelowSimulatePhysics _mesh (Utilities|Name|MakeLiteralName "pelvis") true true))

(fn DisableRagdoll
  (params (Character :type Character%20Object%20Reference))
  (bind _mesh (Variables|/Script/Engine.Character|GetMesh Character))
  (Collision|SetCollisionProfileName _mesh "CharacterMesh" true :!class /Script/Engine.PrimitiveComponent)
  (Physics|SetSimulatePhysics _mesh false)
  (Collision|SetCollisionEnabled (Variables|/Script/Engine.Character|GetCapsuleComponent Character) "QueryAndPhysics"))

(fn CanbeInteracted?
  (params (Actor :type Actor%20Object%20Reference) (CanBe%20Check :type Boolean))
  (if (Object|IsObjectEmpty Actor true)
    (if (Utilities|DoesObjectImplementInterface Actor "/Game/RPGCharacterCreator/Blueprints/BPI_InteractionInterface.BPI_InteractionInterface_C")
      (if CanBe%20Check
        (bind _can_ (Class|BPIInteractionInterface|ICanbeInteracted(Message) Actor))
        (if _can_
          (return true)
          (else
            (return false)))
        (else
          (return true)))
      (else
        _)))
  (return false))

(fn If1Then0
  (params (Input :type Integer))
  (if (== Input 1)
    (return 0)
    (else
      (return Input))))

(fn GetEmptyColor
  (return (LocalVariables|GetemptyColor)))

(fn NameEmpty
  (params (String :type Name) (Not :type Boolean))
  (bind _returnvalue (Utilities|Name|Equal(Name) String "None"))
  (bind _returnvalue_2 (Utilities|Name|Equal(Name) String ""))
  (bind _returnvalue_3 (or _returnvalue_2 _returnvalue))
  (if Not
    (return (not _returnvalue_3))
    (else
      (return _returnvalue_3))))

(fn HasStaticMesh
  (params (Slot :type Static%20Mesh%20Component%20Object%20Reference))
  (bind _isempty_ (Object|IsObjectEmpty Slot true))
  (if _isempty_
    (return (Object|IsObjectEmpty (Variables|/Script/Engine.StaticMeshComponent|GetStaticMesh Slot) true))
    (else
      (return _isempty_))))

(fn HasSkeletalMesh
  (params (Slot :type Skeletal%20Mesh%20Component%20Object%20Reference))
  (bind _isempty_ (Object|IsObjectEmpty Slot true))
  (if _isempty_
    (return (Object|IsObjectEmpty (Variables|/Script/Engine.SkinnedMeshComponent|GetSkeletalMesh Slot) true))
    (else
      (return _isempty_))))

(fn GetPrimitiveMaterialSlotNames
  (params (Primitive :type Primitive%20Component%20Object%20Reference))
  (LocalVariables|SetLPrimitive Primitive)
  ;[1 1 1] From Static Mesh Components
  (bind _asstatic_mesh_component (Utilities|Casting|CastToStaticMeshComponent (LocalVariables|GetLPrimitive))
    (:then
      (bind _output_get (LocalVariables|SetLSlotNames (Class|MeshComponent|GetMaterialSlotNames _asstatic_mesh_component)))
      (if (and (Mesh|HasStaticMesh _asstatic_mesh_component) (!= (Utilities|Array|Length _output_get) 0))
        (LocalVariables|SetCMN (Utilities|GetObjectName (Variables|/Script/Engine.StaticMeshComponent|GetStaticMesh _asstatic_mesh_component)))
        (return (LocalVariables|GetLSlotNames) (LocalVariables|GetCMN))))
    (:CastFailed
      ;[1 1 1] From Skeletal Mesh Components
      (bind _asskeletal_mesh_component (Utilities|Casting|CastToSkeletalMeshComponent (LocalVariables|GetLPrimitive))
        (:then
          (bind _output_get_2 (LocalVariables|SetLSlotNames (Class|MeshComponent|GetMaterialSlotNames _asskeletal_mesh_component)))
          (if (and (Mesh|HasSkeletalMesh _asskeletal_mesh_component) (!= (Utilities|Array|Length _output_get_2) 0))
            (LocalVariables|SetCMN (Utilities|GetObjectName (Variables|/Script/Engine.SkinnedMeshComponent|GetSkeletalMesh _asskeletal_mesh_component)))
            (return (LocalVariables|GetLSlotNames) (LocalVariables|GetCMN))))
        (:CastFailed
          (return (LocalVariables|GetLSlotNames) (LocalVariables|GetCMN)))))))

(fn IsMoving
  (params (Primitive :type Primitive%20Component%20Object%20Reference) (Tolerance :type Float%20%28single-precision%29) (Not :type Boolean))
  (bind _returnvalue (Physics|GetPhysicsLinearVelocity Primitive "None"))
  (if Not
    (return (Math|Vector|Equal(Vector) (Math|Vector|Normalize _returnvalue Tolerance) "0, 0, 0" Tolerance))
    (else
      (return (not (Math|Vector|Equal(Vector) (Math|Vector|Normalize _returnvalue Tolerance) "0, 0, 0" Tolerance))))))

(fn CharacterFindFloor
  (params (Character :type Character%20Object%20Reference) (CapsuleLocation :type Vector))
  (bind (_actorcomponent _isfound_) (Component|GetComponent Character "/Script/Engine.CharacterMovementComponent"))
  (if _isfound_
    (bind _ascharacter_movement_component (Utilities|Casting|CastToCharacterMovementComponent _actorcomponent)
      (:then
        (return (.FloorDist (Utilities|Struct|BreakFindFloorResult (Pawn|Components|CharacterMovement|FindFloor _ascharacter_movement_component CapsuleLocation))) (Pawn|Components|CharacterMovement|FindFloor _ascharacter_movement_component CapsuleLocation)))
      (:CastFailed
        _)))
  (return 0.0 ""))

(fn RandomIntNR
  (params (Max :type Integer))
  (bind _indexes (LocalVariables|GetIndexes))
  (if (!= Max 0)
    (for _index (range 0 (- Max 1))
      (Utilities|Array|Add (LocalVariables|GetIndexes) _index))
    (Utilities|Array|Shuffle _indexes)
    (return (Utilities|Array|Get(acopy) _indexes))
    (else
      (return 0))))

(fn GetCleanClassName
  (params (Object :type Object%20Object%20Reference))
  (bind _returnvalue (Utilities|GetClass Object))
  (bind _returnvalue_2 (Utilities|GetClassDisplayName _returnvalue))
  (bind _returnvalue_3 (Utilities|String|FindSubstring _returnvalue_2 "_" false true))
  (bind _returnvalue_4 (Utilities|String|Len _returnvalue_2))
  (bind _returnvalue_5 (- _returnvalue_4 _returnvalue_3))
  (if (> _returnvalue_5 0)
    (return (Utilities|String|Replace _returnvalue_2 (Utilities|String|GetSubstring _returnvalue_2 _returnvalue_3 _returnvalue_5)))
    (else
      (return _returnvalue_2))))

(fn If0Then1Float
  (params (Input :type Float%20%28single-precision%29))
  (if (<= Input 0.0)
    (return 1.0)
    (else
      (return Input))))

(fn GetGravityZ
  (params (PlayerIndex :type Integer))
  (bind _returnvalue (Game|GetPlayerCharacter 0 PlayerIndex))
  (if (Object|IsObjectEmpty _returnvalue true)
    (return (Components|Movement|GetGravityZ (Variables|/Script/Engine.Character|GetCharacterMovement _returnvalue)))
    (else
      (return -9.8e+02))))

(fn FindActiveCameraCharacterComponentRef
  (params (PlayerIndex :type Integer))
  (bind _ascharacter (Utilities|Casting|CastToCharacter (Components|GetOwner (Game|GetPlayerCameraManager 0 PlayerIndex)))
    (:then
      (for _array_element (Components|GetChildrenComponents (Variables|/Script/Engine.Character|GetCapsuleComponent _ascharacter) true)
        (bind _ascamera_component (Utilities|Casting|CastToCameraComponent _array_element))
        (if (Components|Activation|IsActive _ascamera_component)
          (return true _ascamera_component))))
    (:CastFailed
      _))
  (return false 0))

(fn FindCharacterActiveCameraRef
  (params (Character :type Character%20Object%20Reference))
  (for _array_element (Components|GetChildrenComponents (Variables|/Script/Engine.Character|GetCapsuleComponent Character) true)
    (bind _ascamera_component (Utilities|Casting|CastToCameraComponent _array_element))
    (if (Components|Activation|IsActive _ascamera_component)
      (bind _asspring_arm_component (Utilities|Casting|CastToSpringArmComponent (Transformation|GetAttachParent _ascamera_component))
        (:then
          (return true _ascamera_component (Variables|/Script/Engine.SpringArmComponent|GetTargetArmLength _asspring_arm_component)))
        (:CastFailed
          (return true _ascamera_component 0.0)))))
  (return false 0 0.0))

(fn CountSimilarinStringArray
  (params (Array :type Array%20of%20Strings) (StringToSearch :type String))
  (for _array_element Array
    (if (Utilities|Enum|Equal(Enum) _array_element StringToSearch)
      (Math|Integer|IncrementInt (LocalVariables|GetSimilarCount))))
  (return (LocalVariables|GetSimilarCount)))

(fn IsActorFacingCamera?
  (params (Actor :type Actor%20Object%20Reference))
  (bind _returnvalue (Game|GetPlayerCameraManager 0))
  (return (Math|Vector|DotProduct (Math|Vector|Normalize (- (Transformation|GetActorLocation Actor) (Camera|GetCameraLocation _returnvalue))) (Math|Vector|Normalize (Transformation|GetActorForwardVector _returnvalue)))))

(fn GetSkeletalMeshName
  (params (Mesh :type Skeletal%20Mesh%20Component%20Object%20Reference))
  (if (Mesh|HasSkeletalMesh Mesh)
    (return (Utilities|GetObjectName (Variables|/Script/Engine.SkinnedMeshComponent|GetSkeletalMesh Mesh)))
    (else
      (return ""))))

(fn GetStaticMeshName
  (params (Mesh :type Static%20Mesh%20Component%20Object%20Reference))
  (if (Mesh|HasStaticMesh Mesh)
    (return (Utilities|GetObjectName (Variables|/Script/Engine.StaticMeshComponent|GetStaticMesh Mesh)))
    (else
      (return ""))))

(fn GetCleanObjectName
  (params (Object :type Object%20Object%20Reference))
  (bind _returnvalue (Utilities|GetObjectName Object))
  (bind _returnvalue_2 (Utilities|String|FindSubstring _returnvalue "_" false true))
  (bind _returnvalue_3 (Utilities|String|Len _returnvalue))
  (bind _returnvalue_4 (- _returnvalue_3 _returnvalue_2))
  (if (> _returnvalue_4 0)
    (return (Utilities|String|Replace _returnvalue (Utilities|String|GetSubstring _returnvalue _returnvalue_2 _returnvalue_4)))
    (else
      (return _returnvalue))))

(fn IfEmptyThenDefaultString
  (params (String :type String) (Default :type String))
  (if (String|StringEmpty String false)
    (return Default)
    (else
      (return String))))

(fn IfEmptyThenDefaultName
  (params (Imput :type Name) (Default :type Name))
  (if (Name|NameEmpty Imput false)
    (return Default)
    (else
      (return Imput))))

(fn IfInputEqtoThenDefaultInteger
  (params (Input :type Integer) (EqTo :type Integer) (Default :type Integer))
  (if (== Input EqTo)
    (return Default)
    (else
      (return Input))))

(fn GetItemQualityColor
  (params (ItemQuality :type E_ItemQuality%20Enum :default "NewEnumerator0"))
  (switch Utilities|FlowControl|Switch|SwitchonE_ItemQuality ItemQuality
    (:NewEnumerator0
      (return "(R=1.000000,G=1.000000,B=1.000000,A=1.000000)"))
    (:NewEnumerator1
      (return "(R=0.052339,G=0.416667,B=0.000000,A=1.000000)"))
    (:NewEnumerator2
      (return "(R=0.000000,G=0.045322,B=0.395833,A=1.000000)"))
    (:NewEnumerator3
      (return "(R=0.416667,G=0.000000,B=0.326632,A=1.000000)"))
    (:NewEnumerator4
      (return "(R=0.416667,G=0.055854,B=0.000000,A=1.000000)"))))

(fn GetStaticSlotRef
  (params (Eq%20Slot :type ST%20Character%20I%20Equipment%20Slot%20Parameter%20Structure))
  (bind _characterslots (Utilities|Struct|BreakST_CharacterIEquipmentSlotParameter Eq%20Slot))
  (bind _staticslot (Utilities|Struct|BreakST_CharacterSlots _characterslots))
  (return (Object|IsObjectEmpty _staticslot false) _staticslot))

(fn GetSkeletalSlotRef
  (params (Eq%20Slot :type ST%20Character%20I%20Equipment%20Slot%20Parameter%20Structure))
  (bind _characterslots (Utilities|Struct|BreakST_CharacterIEquipmentSlotParameter Eq%20Slot))
  (bind _skeletalslot (Utilities|Struct|BreakST_CharacterSlots _characterslots))
  (return (Object|IsObjectEmpty _skeletalslot false) _skeletalslot))

(fn GetCurrentStacks
  (params (Item :type ST%20Character%20Item%20Structure))
  (return (Math|If0Then1 (.currentitemscount (.Stackable (Utilities|Struct|BreakST_CharacterItem Item))))))

(fn GetMaxStackSize
  (params (Item :type ST%20Character%20Item%20Structure))
  (bind _stackable (Utilities|Struct|BreakST_CharacterItem Item))
  (return (Math|If0Then1 (.maxstacksize _stackable)) (.stackable _stackable)))

(fn GetPrimitiveMeshName
  (params (Primitive :type Primitive%20Component%20Object%20Reference))
  (bind _asskeletal_mesh_component (Utilities|Casting|CastToSkeletalMeshComponent Primitive)
    (:then
      (return (Component|GetSkeletalMeshName _asskeletal_mesh_component)))
    (:CastFailed
      (bind _asstatic_mesh_component (Utilities|Casting|CastToStaticMeshComponent Primitive)
        (:then
          (return (Component|GetStaticMeshName _asstatic_mesh_component)))
        (:CastFailed
          (return ""))))))

(fn IfInputEqtoThenDefaultFloat
  (params (Input :type Float%20%28single-precision%29) (EqTo :type Float%20%28single-precision%29) (Default :type Float%20%28single-precision%29))
  (if (== Input EqTo)
    (return Default)
    (else
      (return Input))))

(fn GetActorDistancetoPlayerCamera
  (params (Actor :type Actor%20Object%20Reference))
  (return (Math|Float|Truncate (Math|Vector|Distance(Vector) (Camera|GetCameraLocation (Game|GetPlayerCameraManager 0)) (Transformation|GetActorLocation Actor)))))