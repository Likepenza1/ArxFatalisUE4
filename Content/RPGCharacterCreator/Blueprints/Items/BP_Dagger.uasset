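; BP_Dagger is a dagger item Blueprint in the RPG Character Creator that extends a parent item class with save-state handling.
; Its save interface function packs the static mesh transform, class, Used flag and current endurance into an actor save struct.
; SaveState passes Used to the parent's version, and LoadState calls the parent before restoring Used.
; The event graph holds only disabled default events, and construction defers to the parent.
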(event EventBeginPlay
  (|CallParentFunction) ; This node is disabled and will not be called.\nDrag off pins to build functionality.
)

(event Collision|EventActorBeginOverlap
  (params (OtherActor :type Actor%20Object%20Reference)))

(event EventTick
  (params (DeltaSeconds :type Float%20%28single-precision%29)))

(fn ConstructionScript
  (|CallParentFunction))

(fn LoadState
  (params (SaveDataAdd :type S%20Save%20Actor%20Structure))
  (|CallParentFunction SaveDataAdd)
  (Variables|Default|SetUsed (.IsOn (Utilities|Struct|BreakS_SaveActor SaveDataAdd))))

(fn SaveState
  (params (Save%20Data%20Add :type S%20Save%20Actor%20Add%20Structure))
  (bind _save_data (|CallParentFunction (Utilities|Struct|MakeS_SaveActorAdd (Utilities|Array|MakeArray (Variables|Default|GetUsed)))))
  (return _save_data))

(fn BPISaveState
  (return (Utilities|Struct|MakeS_SaveActor (Transformation|GetWorldTransform (Variables|Default|GetItemStaticMesh)) (Utilities|GetClass self) (Variables|Default|GetUsed) (Variables|Default|GetEnduranceCurrent))))