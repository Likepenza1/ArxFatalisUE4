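; BP_KeyRing_3 is a key ring item Blueprint in the RPG Character Creator project, built on inherited item behavior.
; It implements BPI_SaveState, packing the static mesh's world transform, its own class, the used flag and current endurance into a save-actor struct.
; The construction script only calls its parent, and the event graph holds just disabled stub events, so it adds no other logic.
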(event EventBeginPlay
  (|CallParentFunction) ; This node is disabled and will not be called.\nDrag off pins to build functionality.
)

(event Collision|EventActorBeginOverlap
  (params (OtherActor :type Actor%20Object%20Reference)))

(event EventTick
  (params (DeltaSeconds :type Float%20%28single-precision%29)))

(fn ConstructionScript
  (|CallParentFunction))

(fn BPISaveState
  (return (Utilities|Struct|MakeS_SaveActor (Transformation|GetWorldTransform (Variables|Default|GetItemStaticMesh)) (Utilities|GetClass self) (Variables|Default|GetUsed) (Variables|Default|GetEnduranceCurrent))))