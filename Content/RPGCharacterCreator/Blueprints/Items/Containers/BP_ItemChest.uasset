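; BP_ItemChest is an interactable loot container that opens the interacting character's loot view and destroys itself once empty.
; On BeginPlay, an empty chest with a LootId fills its items through the player's inventory component loot lookup.
; Interfaces expose items, interaction text and outline highlighting; ending interaction rewinds the skeletal mesh to closed.
; Tick polls the item count to trigger destruction, and the construction script applies the configured static mesh.
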(event EventBeginPlay
  (bind _returnvalue (Game|GetPlayerCharacter 0))
  (bind (_inventory _isfound_) (CallFunction|GetInventoryComponent _returnvalue))
  (|CallParentFunction)
  ;[1 1 1] If Inventory empty - reinitialize it from data table
  (if (and (== (Utilities|Map|Length (Variables|Default|GetInventoryItems)) 0) (CallFunction|NameEmpty (Variables|Default|GetLootId) true))
    (if _isfound_
      (bind (_found_ _trade_item_sell_price_charge _lootitems) (Default|LoadLootbyId _inventory (Variables|Default|GetLootId)))
      (if _found_
        (Variables|Default|SetInventoryItems _lootitems)))))

(event EventTick
  (params (DeltaSeconds :type Float%20%28single-precision%29))
  (if (== (Utilities|Map|Length (Variables|Default|GetInventoryItems)) 0)
    (Actor|DestroyActor)))

(event EventIShowOutline
  (CallFunction|ShowOutline))

(event EventIHideOutline
  (CallFunction|HideOutline))

(fn ConstructionScript
  (|CallParentFunction)
  (Components|StaticMesh|SetStaticMesh (Variables|Default|GetItemStaticMesh) (Variables|Default|GetNew%20Mesh)))

(fn IInteract
  (params (InteractingCharacter :type Character%20Object%20Reference))
  (bind (_inventory _isfound_) (CallFunction|GetInventoryComponent InteractingCharacter))
  (if _isfound_
    (LocalVariables|SetInventoryRef _inventory)
    (Audio|PlaySoundatLocation (Variables|Default|GetOpenSound) "0, 0, 0" "0, 0, 0" 1.0 1.0 0.0 0 0 0)
    (Default|ShowLoot (LocalVariables|GetInventoryRef) self false)
    (return false)))

(fn IGetInventoryItems
  (return (Variables|Default|GetInventoryItems)))

(fn ISetInventoryItems
  (params (Items :type Map%20of%20ST%20Item%20Slot%20Params%20Structures%20to%20Structs))
  (Variables|Default|SetInventoryItems Items)
  (return true))

(fn IEndInteraction
  (params (InteractingCharacter :type Character%20Object%20Reference))
  ;[1 1 1] Close Chest
  (Components|Animation|SetPosition (Variables|Default|GetItemSkeletalMesh) 0.0 true)
  (return true))

(fn ICanbeInteracted
  (return true))

(fn IGetInteractionText
  (bind (_interactiontext _description) (CallFunction|GetInteractionText))
  (if (!= (Utilities|Map|Length (Variables|Default|GetInventoryItems)) 0)
    (return _interactiontext _description)
    (else
      (return _interactiontext "<Empty>"))))

(fn Loot
  (params (ActorOwner :type Actor%20Object%20Reference))
  (bind (_inventory _isfound_) (CallFunction|GetInventoryComponent ActorOwner))
  (if _isfound_
    (LocalVariables|SetInventoryRef _inventory)
    (Default|ShowLoot (LocalVariables|GetInventoryRef) self (Variables|Default|GetCondition))))