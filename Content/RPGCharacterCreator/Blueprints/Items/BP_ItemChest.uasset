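; Lootable chest item for the RPG character creator that opens the interacting character's inventory loot window.
; On BeginPlay an empty chest fills its items from LootId, looked up through the player's inventory component.
; Interaction plays the open sound, shows loot and switches to cursor input, while interface getters and setters expose the items.
; Save and load persist the Used flag and contents; outline events are stubbed and UpdateLoad is disconnected.
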(event EventBeginPlay
  (bind _returnvalue (Game|GetPlayerCharacter 0))
  (bind (_inventory _isfound_) (CallFunction|GetInventoryComponent _returnvalue))
  (|CallParentFunction)
  ;[1 1 1] If Inventory empty - reinitialize it from data table
  (if (and (== (Utilities|Map|Length (Variables|Default|GetInventoryItems)) 0) (CallFunction|NameEmpty (Variables|Default|GetLootId) true))
    (if _isfound_
      (bind (_found_ _trade_item_sell_price_charge _lootitems) (Default|LoadLootbyId _inventory (Variables|Default|GetLootId)))
      (if _found_
        (Variables|Default|SetInventoryItems _lootitems)))))

(event EventIShowOutline)

(event EventIHideOutline)

(fn ConstructionScript
  (|CallParentFunction)
  (Components|StaticMesh|SetStaticMesh (Variables|Default|GetItemStaticMesh) (Variables|Default|GetNew%20Mesh)))

(fn IInteraction
  (params (InteractingCharacter :type Character%20Object%20Reference))
  (bind (_inventory _isfound_) (CallFunction|GetInventoryComponent InteractingCharacter))
  (bind _returnvalue (Game|GetPlayerController 0))
  (if _isfound_
    (LocalVariables|SetInventoryRef _inventory)
    (Audio|PlaySoundatLocation (Variables|Default|GetOpenSound) "0, 0, 0" "0, 0, 0" 1.0 1.0 0.0 0 0 0)
    (Default|ShowLoot (LocalVariables|GetInventoryRef) self false)
    (Input|SetInputModeGameandUI _returnvalue 0 "DoNotLock" false)
    (Variables|/Script/Engine.PlayerController|SetbShowMouseCursor _returnvalue true)
    (Default|HideCursor (CallFunction|--GetPlayerCharacter))
    (return (Variables|Default|GetName) true false)
    (else
      (return (Variables|Default|GetName) true false))))

(fn IGetInventoryItems
  (return (Variables|Default|GetInventoryItems)))

(fn ISetInventoryItems
  (params (Items :type Map%20of%20ST%20Item%20Slot%20Params%20Structures%20to%20Structs))
  (Variables|Default|SetInventoryItems Items)
  (return true))

(fn IEndInteraction
  (params (InteractingCharacter :type Character%20Object%20Reference))
  (return true))

(fn ICanbeInteracted
  (return true))

(fn IGetInteractionText
  (return "" ""))

(fn Loot
  (params (ActorOwner :type Actor%20Object%20Reference))
  (bind (_inventory _isfound_) (CallFunction|GetInventoryComponent ActorOwner))
  (if _isfound_
    (LocalVariables|SetInventoryRef _inventory)
    (Default|ShowLoot (LocalVariables|GetInventoryRef) self (Variables|Default|GetCondition))))

(fn LoadState
  (params (SaveDataAdd :type S%20Save%20Actor%20Structure))
  (bind (_position _classactor _isdead _ison _add _actor _baseitem _container) (Utilities|Struct|BreakS_SaveActor SaveDataAdd))
  (|CallParentFunction SaveDataAdd)
  (Variables|Default|SetUsed _ison)
  (Variables|Default|SetInventoryItems (Utilities|Struct|BreakST_ContainerParam _container)))

(fn SaveState
  (params (Save%20Data%20Add :type S%20Save%20Actor%20Add%20Structure))
  (bind _save_data (|CallParentFunction (Utilities|Struct|MakeS_SaveActorAdd (Utilities|Array|MakeArray (Variables|Default|GetUsed)))))
  (return _save_data))

(fn BPISaveState
  (return (Utilities|Struct|MakeS_SaveActor "0.000000,0.000000,0.000000|0.000000,0.000000,0.000000|1.000000,1.000000,1.000000" 0 false (Variables|Default|GetUsed) (Utilities|Struct|MakeS_SaveActorAdd 0) 0 0 (Utilities|Struct|MakeST_ContainerParam (Variables|Default|GetInventoryItems)))))

(fn UpdateLoad
  (if (== (Utilities|Map|Length (Variables|Default|GetInventoryItems)) 0)
    (Variables|Default|SetUsed true)))