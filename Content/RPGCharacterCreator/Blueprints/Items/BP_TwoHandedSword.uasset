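; Two-handed sword item Blueprint for the RPG character creator that adds save and load of its used flag and endurance.
; BPI_SaveState records the static mesh's world transform, the actor class, Used and current endurance, and LoadState restores Used and endurance after calling the parent.
; SaveState forwards only Used to the parent version.
; BeginPlay and construction just call the parent, with no other logic of its own.
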(event EventBeginPlay
  (|CallParentFunction))

(event Collision|EventActorBeginOverlap
  (params (OtherActor :type Actor%20Object%20Reference)))

(event EventTick
  (params (DeltaSeconds :type Float%20%28single-precision%29)))

(fn ConstructionScript
  (|CallParentFunction))

(fn LoadState
  (params (SaveDataAdd :type S%20Save%20Actor%20Structure))
  (bind (_position _classactor _ison _integer) (Utilities|Struct|BreakS_SaveActor SaveDataAdd))
  (|CallParentFunction SaveDataAdd)
  (Variables|Default|SetUsed _ison)
  (Variables|Default|SetEnduranceCurrent _integer))

(fn SaveState
  (params (Save%20Data%20Add :type S%20Save%20Actor%20Add%20Structure))
  (bind _save_data (|CallParentFunction (Utilities|Struct|MakeS_SaveActorAdd (Utilities|Array|MakeArray (Variables|Default|GetUsed)))))
  (return _save_data))

(fn BPISaveState
  (return (Utilities|Struct|MakeS_SaveActor (Transformation|GetWorldTransform (Variables|Default|GetItemStaticMesh)) (Utilities|GetClass self) (Variables|Default|GetUsed) (Variables|Default|GetEnduranceCurrent))))