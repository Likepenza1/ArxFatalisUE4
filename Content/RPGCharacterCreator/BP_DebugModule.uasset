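; Debug component for the RPG character creator that shows the WB_Debug overlay for player-controlled characters.
; On BeginPlay, if debugging is enabled and the inverted IsNPC check passes, Initialize caches the owning Character and its mesh, then ShowUi adds the widget to the first player's screen.
; IsNPC has a fallback for non-Pawn owners based on BP_FreeCamera, though initialization still requires a Character owner.
; HideUi removes the stored widget.
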(event EventBeginPlay
  (bind _isnpc_ (Main|IsNPC true))
  (if (and _isnpc_ (Variables|Settings|GetEnable%20Debug))
    (Main|Initialize)))

(fn Initialize
  (Utilities|FlowControl|Sequence
    (:then_0
      ;[1 1 1] Checks
      (bind _ascharacter (Utilities|Casting|CastToCharacter (Components|GetOwner))
        (:then
          (Variables|Character|SetOwner _ascharacter)
          (if (CallFunction|IsObjectEmpty (Variables|/Script/Engine.Character|GetMesh _ascharacter) true)
            (Variables|Character|SetCharacterMesh (Variables|/Script/Engine.Character|GetMesh _ascharacter))
            (else
              ;;[1 0.009645 0] Can't initialise
              (bind _output_get (Variables|Local|SetIsInitialized? false :!label _label))
              (return _output_get))))
        (:CastFailed
          (goto _label))))
    (:then_1
      ;[1 1 1] Show UI
      (bind _isnpc_ (Main|IsNPC true))
      (if _isnpc_
        (Ui|ShowUi)))
    (:then_2
      ;[1 0 0.07331] Return
      (bind _output_get_2 (Variables|Local|SetIsInitialized? true))
      (return _output_get_2))))

(fn ShowUi
  (bind _returnvalue (UserInterface|CreateWidget "/Game/RPGCharacterCreator/UI/WB_Debug.WB_Debug_C" (Game|GetPlayerController 0) (Variables|Character|GetOwner)))
  (bind _returnvalue_2 (UserInterface|Viewport|AddtoPlayerScreen _returnvalue (Variables|Settings|GetWidgetOverlayZIndex)))
  (if _returnvalue_2
    (bind _output_get (Variables|Ui|SetUiWidget _returnvalue))
    (return true _output_get)
    (else
      (return false 0))))

(fn HideUi
  (bind (_valid_ _uiwidget) (Ui|Pure|GetBaseUi))
  (if _valid_
    (Widget|RemovefromParent _uiwidget)))

(fn GetBaseUi
  (bind _uiwidget (Variables|Ui|GetUiWidget))
  (if (CallFunction|IsObjectEmpty _uiwidget true)
    (return true _uiwidget)
    (else
      (return false 0))))

(fn IsNPC
  (params (Not :type Boolean))
  (bind _aspawn (Utilities|Casting|CastToPawn (Components|GetOwner))
    (:then
      (if Not
        (return (Pawn|IsPlayerControlled _aspawn))
        (else
          (return (not (Pawn|IsPlayerControlled _aspawn))))))
    (:CastFailed
      (Utilities|Casting|CastToBP_FreeCamera (Game|Player|GetPlayerPawn 0)
        (:then
          (if Not
            (return true)
            (else
              (return false))))
        (:CastFailed
          (return (not Not)))))))

(fn IsInitialized
  (params (Not :type Boolean))
  (bind _isinitialized_ (Variables|Local|GetIsInitialized?))
  (if Not
    (return (not _isinitialized_))
    (else
      (return _isinitialized_))))