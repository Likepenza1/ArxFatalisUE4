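; Game instance that saves and loads the game through an Arx_SaveGame object in a named slot.
; It stores player transform, camera rotation, weapon mode, base stats, six runes, and inventory with equipment and action bar.
; Level actors implementing BPI_SaveLoadd supply their own state, stored by object name.
; Loading matches those names, then sends every such actor a load-done message, and re-equips items before syncing inventory UI.
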(fn Save
  (bind _returnvalue (SaveGame|CreateSaveGameObject "/Game/Blueprints/SaveGame/Arx_SaveGame.Arx_SaveGame_C"))
  (Variables|Default|SetSaveGame _returnvalue)
  (SaveCategory|SaveInventory)
  (SaveCategory|SavePlayer)
  (SaveCategory|SaveLevel)
  (SaveCategory|SaveRune)
  (SaveGame|SaveGametoSlot (Variables|Default|GetSaveGame) (Variables|Default|GetSaveSlotName))
  (Development|PrintString "Save Game!"))

(fn SaveLevel
  (bind _savegame (Variables|Default|GetSaveGame))
  (bind _actorsall (Variables|/Game/Blueprints/SaveGame/Arx_SaveGame.Arx_SaveGame_C|GetActorsAll _savegame))
  (bind _outactors (Actor|GetAllActorswithInterface "/Game/Blueprints/SaveGame/BPI_SaveLoadd.BPI_SaveLoadd_C"))
  (Utilities|Map|Clear _actorsall)
  (for _array_element _outactors
    (bind _saveslot (Class|BPISaveLoadd|BPISaveState(Message) _array_element))
    (Utilities|Map|Add _actorsall (Utilities|GetObjectName _array_element) _saveslot))
  (return))

(fn Load
  (bind _returnvalue (SaveGame|LoadGamefromSlot (Variables|Default|GetSaveSlotName)))
  (bind _asarx_save_game (Utilities|Casting|CastToArx_SaveGame _returnvalue))
  (Variables|Default|SetSaveGame _asarx_save_game)
  (LoadCategory|LoadInventory)
  (LoadCategory|LoadPlayer)
  (LoadCategory|LoadLevel)
  (LoadCategory|LoadRune)
  (Development|PrintString "Load Game!"))

(fn LoadLevel
  (bind _savegame (Variables|Default|GetSaveGame))
  (bind _actorsall (Variables|/Game/Blueprints/SaveGame/Arx_SaveGame.Arx_SaveGame_C|GetActorsAll _savegame))
  (bind _outactors (Actor|GetAllActorswithInterface "/Game/Blueprints/SaveGame/BPI_SaveLoadd.BPI_SaveLoadd_C"))
  (bind _keys (Utilities|Map|Keys _actorsall))
  (for _array_element _keys
    (bind _array_element_2 (Utilities|Array|ForEachLoopwithBreak _outactors :!label _label)
      (:LoopBody
        (LocalVariables|SetLoadActorSuccess false)
        (if (Utilities|Enum|Equal(Enum) _array_element (Utilities|GetObjectName _array_element_2))
          (LocalVariables|SetLoadActorSuccess true)
          (Class|BPISaveLoadd|BPILoadState(Message) _array_element_2 (.Value (Utilities|Map|Find _actorsall _array_element)))
          (goto _label Break)))))
  (bind _outactors_2 (Actor|GetAllActorswithInterface "/Game/Blueprints/SaveGame/BPI_SaveLoadd.BPI_SaveLoadd_C"))
  (for _array_element_3 _outactors_2
    (Class|BPISaveLoadd|BPILoadDone(Message) _array_element_3)))

(fn SavePlayer
  (Variables|/Game/Blueprints/SaveGame/Arx_SaveGame.Arx_SaveGame_C|SetPlayerLocation (Variables|Default|GetSaveGame) (Transformation|GetActorTransform (CallFunction|--GetPlayerCharacter)))
  (Variables|/Game/Blueprints/SaveGame/Arx_SaveGame.Arx_SaveGame_C|SetRotationCamera (Variables|Default|GetSaveGame) (Camera|GetCameraRotation (Game|GetPlayerCameraManager 0)))
  (SaveCategory|SaveStats)
  (Variables|/Game/Blueprints/SaveGame/Arx_SaveGame.Arx_SaveGame_C|SetWeaponMode (Variables|Default|GetSaveGame) (Variables|/Game/RPGCharacterCreator/Blueprints/BP_RPG_CharacterMain.BP_RPG_CharacterMain_C|GetWeaponMod (CallFunction|--GetPlayerCharacter))))

(fn LoadPlayer
  (Transformation|SetActorTransform (CallFunction|--GetPlayerCharacter) (Variables|/Game/Blueprints/SaveGame/Arx_SaveGame.Arx_SaveGame_C|GetPlayerLocation (Variables|Default|GetSaveGame)))
  (Pawn|SetControlRotation (Game|GetPlayerController 0) (Variables|/Game/Blueprints/SaveGame/Arx_SaveGame.Arx_SaveGame_C|GetRotationCamera (Variables|Default|GetSaveGame)))
  (LoadCategory|LoadStats)
  (Variables|/Game/RPGCharacterCreator/Blueprints/BP_RPG_CharacterMain.BP_RPG_CharacterMain_C|SetWeaponMod (CallFunction|--GetPlayerCharacter) (Variables|/Game/Blueprints/SaveGame/Arx_SaveGame.Arx_SaveGame_C|GetWeaponMode (Variables|Default|GetSaveGame))))

(fn SaveStats
  (bind _mycharacter (CallFunction|--GetPlayerCharacter))
  (bind _savegame (Variables|Default|GetSaveGame))
  (bind _bp_stats (Variables|/Game/RPGCharacterCreator/Blueprints/BP_RPG_CharacterMain.BP_RPG_CharacterMain_C|GetBP_Stats _mycharacter))
  (Variables|/Game/Blueprints/SaveGame/Arx_SaveGame.Arx_SaveGame_C|SetStatsValueZdorovie _savegame (Math|Conversions|ToFloat(Integer) (.Value (Default|GetStatValue _bp_stats "NewEnumerator1" false))))
  (Variables|/Game/Blueprints/SaveGame/Arx_SaveGame.Arx_SaveGame_C|SetStatsValueMagicEnergiya _savegame (Math|Conversions|ToFloat(Integer) (.Value (Default|GetStatValue _bp_stats "NewEnumerator3" false))))
  (Variables|/Game/Blueprints/SaveGame/Arx_SaveGame.Arx_SaveGame_C|SetStatsValueDamage _savegame (Math|Conversions|ToFloat(Integer) (.Value (Default|GetStatValue _bp_stats "NewEnumerator4" false))))
  (Variables|/Game/Blueprints/SaveGame/Arx_SaveGame.Arx_SaveGame_C|SetStatsValueZasita _savegame (Math|Conversions|ToFloat(Integer) (.Value (Default|GetStatValue _bp_stats "NewEnumerator5" false))))
  (Variables|/Game/Blueprints/SaveGame/Arx_SaveGame.Arx_SaveGame_C|SetStatsValueVinoslivost _savegame (Math|Conversions|ToFloat(Integer) (.Value (Default|GetStatValue _bp_stats "NewEnumerator37" false))))
  (Variables|/Game/Blueprints/SaveGame/Arx_SaveGame.Arx_SaveGame_C|SetStatsValueSila _savegame (Math|Conversions|ToFloat(Integer) (.Value (Default|GetStatValue _bp_stats "NewEnumerator15" false))))
  (Variables|/Game/Blueprints/SaveGame/Arx_SaveGame.Arx_SaveGame_C|SetStatsValueRazum _savegame (Math|Conversions|ToFloat(Integer) (.Value (Default|GetStatValue _bp_stats "NewEnumerator16" false))))
  (Variables|/Game/Blueprints/SaveGame/Arx_SaveGame.Arx_SaveGame_C|SetStatsValueLovkost _savegame (Math|Conversions|ToFloat(Integer) (.Value (Default|GetStatValue _bp_stats "NewEnumerator31" false))))
  (Variables|/Game/Blueprints/SaveGame/Arx_SaveGame.Arx_SaveGame_C|SetStatsValueNezametnost _savegame (Math|Conversions|ToFloat(Integer) (.Value (Default|GetStatValue _bp_stats "NewEnumerator19" false))))
  (Variables|/Game/Blueprints/SaveGame/Arx_SaveGame.Arx_SaveGame_C|SetStatsValueMehanika _savegame (Math|Conversions|ToFloat(Integer) (.Value (Default|GetStatValue _bp_stats "NewEnumerator20" false))))
  (Variables|/Game/Blueprints/SaveGame/Arx_SaveGame.Arx_SaveGame_C|SetStatsValueIntuition _savegame (Math|Conversions|ToFloat(Integer) (.Value (Default|GetStatValue _bp_stats "NewEnumerator21" false))))
  (Variables|/Game/Blueprints/SaveGame/Arx_SaveGame.Arx_SaveGame_C|SetStatsValueMeditation _savegame (Math|Conversions|ToFloat(Integer) (.Value (Default|GetStatValue _bp_stats "NewEnumerator22" false))))
  (Variables|/Game/Blueprints/SaveGame/Arx_SaveGame.Arx_SaveGame_C|SetStatsValueRemeslo _savegame (Math|Conversions|ToFloat(Integer) (.Value (Default|GetStatValue _bp_stats "NewEnumerator23" false))))
  (Variables|/Game/Blueprints/SaveGame/Arx_SaveGame.Arx_SaveGame_C|SetStatsValueMagia _savegame (Math|Conversions|ToFloat(Integer) (.Value (Default|GetStatValue _bp_stats "NewEnumerator32" false))))
  (Variables|/Game/Blueprints/SaveGame/Arx_SaveGame.Arx_SaveGame_C|SetStatsValueBlizniyBoy _savegame (Math|Conversions|ToFloat(Integer) (.Value (Default|GetStatValue _bp_stats "NewEnumerator33" false))))
  (Variables|/Game/Blueprints/SaveGame/Arx_SaveGame.Arx_SaveGame_C|SetStatsValueStrelba _savegame (Math|Conversions|ToFloat(Integer) (.Value (Default|GetStatValue _bp_stats "NewEnumerator26" false))))
  (Variables|/Game/Blueprints/SaveGame/Arx_SaveGame.Arx_SaveGame_C|SetStatsValueKlassZasiti _savegame (Math|Conversions|ToFloat(Integer) (.Value (Default|GetStatValue _bp_stats "NewEnumerator34" false))))
  (Variables|/Game/Blueprints/SaveGame/Arx_SaveGame.Arx_SaveGame_C|SetStatsValueUstKMagii _savegame (Math|Conversions|ToFloat(Integer) (.Value (Default|GetStatValue _bp_stats "NewEnumerator35" false))))
  (Variables|/Game/Blueprints/SaveGame/Arx_SaveGame.Arx_SaveGame_C|SetStatsValueUstKYadam _savegame (Math|Conversions|ToFloat(Integer) (.Value (Default|GetStatValue _bp_stats "NewEnumerator36" false)))))

(fn LoadStats
  (bind _mycharacter (CallFunction|--GetPlayerCharacter))
  (bind _savegame (Variables|Default|GetSaveGame))
  (bind _bp_stats (Variables|/Game/RPGCharacterCreator/Blueprints/BP_RPG_CharacterMain.BP_RPG_CharacterMain_C|GetBP_Stats _mycharacter))
  (Default|ChangeStatBaseValue _bp_stats "NewEnumerator1" (Math|Float|Truncate (Variables|/Game/Blueprints/SaveGame/Arx_SaveGame.Arx_SaveGame_C|GetStatsValueZdorovie _savegame)))
  (Default|ChangeStatBaseValue _bp_stats "NewEnumerator3" (Math|Float|Truncate (Variables|/Game/Blueprints/SaveGame/Arx_SaveGame.Arx_SaveGame_C|GetStatsValueMagicEnergiya _savegame)))
  (Default|ChangeStatBaseValue _bp_stats "NewEnumerator4" (Math|Float|Truncate (Variables|/Game/Blueprints/SaveGame/Arx_SaveGame.Arx_SaveGame_C|GetStatsValueDamage _savegame)))
  (Default|ChangeStatBaseValue _bp_stats "NewEnumerator5" (Math|Float|Truncate (Variables|/Game/Blueprints/SaveGame/Arx_SaveGame.Arx_SaveGame_C|GetStatsValueZasita _savegame)))
  (Default|ChangeStatBaseValue _bp_stats "NewEnumerator37" (Math|Float|Truncate (Variables|/Game/Blueprints/SaveGame/Arx_SaveGame.Arx_SaveGame_C|GetStatsValueVinoslivost _savegame)))
  (Default|ChangeStatBaseValue _bp_stats "NewEnumerator15" (Math|Float|Truncate (Variables|/Game/Blueprints/SaveGame/Arx_SaveGame.Arx_SaveGame_C|GetStatsValueSila _savegame)))
  (Default|ChangeStatBaseValue _bp_stats "NewEnumerator16" (Math|Float|Truncate (Variables|/Game/Blueprints/SaveGame/Arx_SaveGame.Arx_SaveGame_C|GetStatsValueRazum _savegame)))
  (Default|ChangeStatBaseValue _bp_stats "NewEnumerator31" (Math|Float|Truncate (Variables|/Game/Blueprints/SaveGame/Arx_SaveGame.Arx_SaveGame_C|GetStatsValueLovkost _savegame)))
  (Default|ChangeStatBaseValue _bp_stats "NewEnumerator19" (Math|Float|Truncate (Variables|/Game/Blueprints/SaveGame/Arx_SaveGame.Arx_SaveGame_C|GetStatsValueNezametnost _savegame)))
  (Default|ChangeStatBaseValue _bp_stats "NewEnumerator20" (Math|Float|Truncate (Variables|/Game/Blueprints/SaveGame/Arx_SaveGame.Arx_SaveGame_C|GetStatsValueMehanika _savegame)))
  (Default|ChangeStatBaseValue _bp_stats "NewEnumerator21" (Math|Float|Truncate (Variables|/Game/Blueprints/SaveGame/Arx_SaveGame.Arx_SaveGame_C|GetStatsValueIntuition _savegame)))
  (Default|ChangeStatBaseValue _bp_stats "NewEnumerator22" (Math|Float|Truncate (Variables|/Game/Blueprints/SaveGame/Arx_SaveGame.Arx_SaveGame_C|GetStatsValueMeditation _savegame)))
  (Default|ChangeStatBaseValue _bp_stats "NewEnumerator23" (Math|Float|Truncate (Variables|/Game/Blueprints/SaveGame/Arx_SaveGame.Arx_SaveGame_C|GetStatsValueRemeslo _savegame)))
  (Default|ChangeStatBaseValue _bp_stats "NewEnumerator32" (Math|Float|Truncate (Variables|/Game/Blueprints/SaveGame/Arx_SaveGame.Arx_SaveGame_C|GetStatsValueMagia _savegame)))
  (Default|ChangeStatBaseValue _bp_stats "NewEnumerator33" (Math|Float|Truncate (Variables|/Game/Blueprints/SaveGame/Arx_SaveGame.Arx_SaveGame_C|GetStatsValueBlizniyBoy _savegame)))
  (Default|ChangeStatBaseValue _bp_stats "NewEnumerator26" (Math|Float|Truncate (Variables|/Game/Blueprints/SaveGame/Arx_SaveGame.Arx_SaveGame_C|GetStatsValueStrelba _savegame)))
  (Default|ChangeStatBaseValue _bp_stats "NewEnumerator34" (Math|Float|Truncate (Variables|/Game/Blueprints/SaveGame/Arx_SaveGame.Arx_SaveGame_C|GetStatsValueKlassZasiti _savegame)))
  (Default|ChangeStatBaseValue _bp_stats "NewEnumerator35" (Math|Float|Truncate (Variables|/Game/Blueprints/SaveGame/Arx_SaveGame.Arx_SaveGame_C|GetStatsValueUstKMagii _savegame)))
  (Default|ChangeStatBaseValue _bp_stats "NewEnumerator36" (Math|Float|Truncate (Variables|/Game/Blueprints/SaveGame/Arx_SaveGame.Arx_SaveGame_C|GetStatsValueUstKYadam _savegame))))

(fn SaveRune
  (bind _mycharacter (CallFunction|--GetPlayerCharacter))
  (bind _savegame (Variables|Default|GetSaveGame))
  (Variables|/Game/Blueprints/SaveGame/Arx_SaveGame.Arx_SaveGame_C|SetAam _savegame (Variables|/Game/RPGCharacterCreator/Blueprints/BP_RPG_CharacterMain.BP_RPG_CharacterMain_C|GetAam _mycharacter))
  (Variables|/Game/Blueprints/SaveGame/Arx_SaveGame.Arx_SaveGame_C|SetFolgora _savegame (Variables|/Game/RPGCharacterCreator/Blueprints/BP_RPG_CharacterMain.BP_RPG_CharacterMain_C|GetFolgora _mycharacter))
  (Variables|/Game/Blueprints/SaveGame/Arx_SaveGame.Arx_SaveGame_C|SetMovis _savegame (Variables|/Game/RPGCharacterCreator/Blueprints/BP_RPG_CharacterMain.BP_RPG_CharacterMain_C|GetMovis _mycharacter))
  (Variables|/Game/Blueprints/SaveGame/Arx_SaveGame.Arx_SaveGame_C|SetTaar _savegame (Variables|/Game/RPGCharacterCreator/Blueprints/BP_RPG_CharacterMain.BP_RPG_CharacterMain_C|GetTaar _mycharacter))
  (Variables|/Game/Blueprints/SaveGame/Arx_SaveGame.Arx_SaveGame_C|SetVitae _savegame (Variables|/Game/RPGCharacterCreator/Blueprints/BP_RPG_CharacterMain.BP_RPG_CharacterMain_C|GetVitae _mycharacter))
  (Variables|/Game/Blueprints/SaveGame/Arx_SaveGame.Arx_SaveGame_C|SetYok _savegame (Variables|/Game/RPGCharacterCreator/Blueprints/BP_RPG_CharacterMain.BP_RPG_CharacterMain_C|GetYok _mycharacter)))

(fn LoadRune
  (bind _mycharacter (CallFunction|--GetPlayerCharacter))
  (bind _savegame (Variables|Default|GetSaveGame))
  (Variables|/Game/RPGCharacterCreator/Blueprints/BP_RPG_CharacterMain.BP_RPG_CharacterMain_C|SetAam _mycharacter (Variables|/Game/Blueprints/SaveGame/Arx_SaveGame.Arx_SaveGame_C|GetAam _savegame))
  (Variables|/Game/RPGCharacterCreator/Blueprints/BP_RPG_CharacterMain.BP_RPG_CharacterMain_C|SetFolgora _mycharacter (Variables|/Game/Blueprints/SaveGame/Arx_SaveGame.Arx_SaveGame_C|GetFolgora _savegame))
  (Variables|/Game/RPGCharacterCreator/Blueprints/BP_RPG_CharacterMain.BP_RPG_CharacterMain_C|SetMovis _mycharacter (Variables|/Game/Blueprints/SaveGame/Arx_SaveGame.Arx_SaveGame_C|GetMovis _savegame))
  (Variables|/Game/RPGCharacterCreator/Blueprints/BP_RPG_CharacterMain.BP_RPG_CharacterMain_C|SetTaar _mycharacter (Variables|/Game/Blueprints/SaveGame/Arx_SaveGame.Arx_SaveGame_C|GetTaar _savegame))
  (Variables|/Game/RPGCharacterCreator/Blueprints/BP_RPG_CharacterMain.BP_RPG_CharacterMain_C|SetVitae _mycharacter (Variables|/Game/Blueprints/SaveGame/Arx_SaveGame.Arx_SaveGame_C|GetVitae _savegame))
  (Variables|/Game/RPGCharacterCreator/Blueprints/BP_RPG_CharacterMain.BP_RPG_CharacterMain_C|SetYok _mycharacter (Variables|/Game/Blueprints/SaveGame/Arx_SaveGame.Arx_SaveGame_C|GetYok _savegame)))

(fn SaveInventory
  (bind _mycharacter (CallFunction|--GetPlayerCharacter))
  (bind (_inventory _isfound_) (CallFunction|GetInventoryComponent _mycharacter))
  (Utilities|FlowControl|Sequence
    (:then_0
      ;[0 0.6805 1] Inventory, Action Bar, Equipment
      (if _isfound_
        (bind _total_items (Default|GetEquippedItems _inventory))
        (Utilities|Struct|SetmembersinST_CharacterSettings (LocalVariables|GetCharacterSettings) (Default|GetInventoryItems _inventory) _total_items (Default|GetActionBarSlots _inventory))))
    (:then_1
      ;[1 0.07126 0] Save
      (Variables|/Game/Blueprints/SaveGame/Arx_SaveGame.Arx_SaveGame_C|SetCharacterCustomizerData (Variables|Default|GetSaveGame) (LocalVariables|GetCharacterSettings)))))

(fn LoadInventory
  (bind _mycharacter (CallFunction|--GetPlayerCharacter))
  (bind (_inventory _isfound_) (CallFunction|GetInventoryComponent _mycharacter))
  (LocalVariables|SetCharacterCustomizationData (Variables|/Game/Blueprints/SaveGame/Arx_SaveGame.Arx_SaveGame_C|GetCharacterCustomizerData (Variables|Default|GetSaveGame)))
  (Utilities|FlowControl|Sequence
    (:then_0
      ;[1 1 1] Reinit Inventory Module. this will automatically load all saved data
      (if _isfound_
        (Default|SetInventoryItems _inventory (.InventoryItems (Utilities|Struct|BreakST_CharacterSettings (LocalVariables|GetCharacterCustomizationData))))
        (Variables|/Game/RPGCharacterCreator/Blueprints/BP_InventoryModule.BP_InventoryModule_C|SetActionBarSlots _inventory (.ActionBarItems (Utilities|Struct|BreakST_CharacterSettings (LocalVariables|GetCharacterCustomizationData))))
        (Default|ClearEquippedItems _inventory false false (Utilities|Array|MakeArray))
        (for _array_element (.EquippedItems (Utilities|Struct|BreakST_CharacterSettings (LocalVariables|GetCharacterCustomizationData)))
          (bind _success_ (Default|EquipItem _inventory _array_element false false true)))
        (Default|UpdateCharacterEquipment _inventory)
        (Default|SyncInventoryUI _inventory)))
    (:then_1
      ;[1 0 0] Return
      (return))))