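; Game save component that stores and restores Gold, EXP and the player character.
; Tick polls configurable save and load keys, and BeginPlay runs the same load path automatically.
; Gold and EXP go through an Arx_SaveGame slot, falling back to zero without a valid save, while the character uses a separate "Inventory" slot.
; Each key-driven save and each load also calls the matching Save or Load on ArxInstance.
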(event EventBeginPlay
  ;[1 0.5026 0] If the selected "Load Key" is pressed, load the game.
  (bind (_gold _exp) (CallFunction|LoadGame))
  (CallFunction|SetAllVariables _gold _exp)
  (Default|Load (CallFunction|--ArxInstance)))

(event EventTick
  (params (DeltaSeconds :type Float%20%28single-precision%29))
  ;[1 0.5026 0] If the selected "Save Key" is pressed, save the game.
  (Utilities|FlowControl|Sequence
    (:then_0
      (if (Game|Player|WasInputKeyJustPressed (Game|GetPlayerController 0) (Variables|Default|GetSaveKey))
        (bind (_gold _exp) (CallFunction|GetAllVariables))
        (CallFunction|SaveGame _gold _exp)
        (Default|Save (CallFunction|--ArxInstance))))
    (:then_1
      ;[1 0.5026 0] If the selected "Load Key" is pressed, load the game.
      (if (Game|Player|WasInputKeyJustPressed (Game|GetPlayerController 0) (Variables|Default|GetLoadKey))
        (bind (_gold_2 _exp_2) (CallFunction|LoadGame))
        (CallFunction|SetAllVariables _gold_2 _exp_2)
        (Default|Load (CallFunction|--ArxInstance))))))

(fn SetAllVariables
  (params (Gold :type Integer) (EXP :type Float%20%28single-precision%29))
  ;[1 0.636 0] Sets all of the variables Based on their current value.
  (Variables|Default|SetGold Gold)
  (Variables|Default|SetEXP EXP))

(fn LoadGame
  (CallFunction|LoadCharacterSave (CallFunction|--GetPlayerCharacter) "Inventory")
  ;[1 0.4212 0] First, it checks if a save game exists.
  (bind _returnvalue (SaveGame|DoesSaveGameExist "All Save Information"))
  (if _returnvalue
    ;[1 0.4212 0] If a save game does exist, cast to the save info, if not, then set eveything to it's default value.
    (bind _returnvalue_2 (SaveGame|LoadGamefromSlot "All Save Information"))
    (bind _asarx_save_game (Utilities|Casting|CastToArx_SaveGame _returnvalue_2)
      (:then
        ;[1 0.4212 0] Last it gets all of the variables and sets them in the return node, telling it what values to load.
        (return (Variables|/Game/Blueprints/SaveGame/Arx_SaveGame.Arx_SaveGame_C|GetGold _asarx_save_game) (Variables|/Game/Blueprints/SaveGame/Arx_SaveGame.Arx_SaveGame_C|GetEXP _asarx_save_game)))
      (:CastFailed
        _)))
  ;;[1 0.4212 0] Set all of the variables to Defaults.
  (return 0 0.0))

(fn SaveGame
  (params (Gold :type Integer) (EXP :type Float%20%28single-precision%29))
  ;[1 0.4212 0] First, the save function is getting everything that we want to save.
  ;[1 0.4212 0] Next, it is creating a save game object. (A save file.)
  (bind _returnvalue (SaveGame|CreateSaveGameObject "/Game/Blueprints/SaveGame/Arx_SaveGame.Arx_SaveGame_C"))
  ;[1 0.4212 0] Then, it is setting an information variable and casting to the SaveInfo Blueprint.
  (bind _output_get (Variables|Default|SetInformation _returnvalue))
  ;;[1 0.4212 0] Ignore the note that it gives you. This is necessary
  (bind _asarx_save_game (Utilities|Casting|CastToArx_SaveGame _output_get))
  ;[1 0.421 0] This is where it looks complicated. It is actually pretty straight forward. It is setting all of the variables in our SaveInfo Blueprint based on their variable value. The target is the SaveInfo and the variable base is connected to the function variable setting. WIth a little practice, these can also be implimented into saving other world actors too.
  (Variables|/Game/Blueprints/SaveGame/Arx_SaveGame.Arx_SaveGame_C|SetGold _asarx_save_game Gold)
  (Variables|/Game/Blueprints/SaveGame/Arx_SaveGame.Arx_SaveGame_C|SetEXP _asarx_save_game EXP)
  ;[1 0.421 0] Here it is saving the information to a slot.
  (CallFunction|SaveCharacter (CallFunction|--GetPlayerCharacter) true "Inventory")
  (bind _returnvalue_2 (SaveGame|SaveGametoSlot (Variables|Default|GetInformation) "All Save Information"))
  ;[1 0.421 0] Now it is checking if the save was a success. If it was it will print a string to screen saying that the game save was successful. If the save was unsuccessful, it is printing a string to the screen sayinf that the game save was not successful.
  (if _returnvalue_2
    (Development|PrintString "Game Saved")
    (else
      (Development|PrintString "There was an Error Saving the Game"))))

(fn GetAllVariables
  ;[0.9219 0.3863 0] This simply collects all of the values and sets them into one function, that way they are easier to access.
  (return (Variables|Default|GetGold) (Variables|Default|GetEXP)))