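; BP_Stats manages character stats as an array of base, modifier and max values, with damage rolled from a random critical chance.
; Modifier and base-value edits fire dispatchers, while StatChanged adds or subtracts base values, clamping at zero or max.
; Attribute functions, including Razum and Lovkost, push changes through StatChanged, some indexed by attribute level.
; GetStatValue's IncludeModifiers flag is inverted: false returns base plus modifiers.
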(fn RemoveModifier
  (params (Type :type E_PlayerStats%20Enum :default "NewEnumerator0") (Value :type Float%20%28single-precision%29))
  (if (!= Value 0.0)
    (bind _output_get (LocalVariables|SetL_Index (Stats|GetStatIndex Type)))
    (if (>= _output_get 0)
      (Utilities|Struct|SetmembersinS_Stat (Utilities|Array|Get(acopy) (Variables|Default|GetStat) (LocalVariables|GetL_Index)) (- (Utilities|Struct|BreakS_Stat (Utilities|Array|Get(acopy) (Variables|Default|GetStat) (LocalVariables|GetL_Index))) Value))
      (Default|CallOnModifierRemoved Type Value))))

(fn AddModifier
  (params (Type :type E_PlayerStats%20Enum :default "NewEnumerator0") (Value :type Float%20%28single-precision%29))
  (if (!= Value 0.0)
    (bind _output_get (LocalVariables|SetL_Index (Stats|GetStatIndex Type)))
    (if (>= _output_get 0)
      (Utilities|Struct|SetmembersinS_Stat (Utilities|Array|Get(acopy) (Variables|Default|GetStat) (LocalVariables|GetL_Index)) (+ (.ModifiersValue (Utilities|Struct|BreakS_Stat (Utilities|Array|Get(acopy) (Variables|Default|GetStat) (LocalVariables|GetL_Index)))) Value))
      (Default|CallOnModifierAdded Type Value))))

(fn ChangeStatBaseValue
  (params (Type :type E_PlayerStats%20Enum :default "NewEnumerator0") (NewValue :type Float%20%28single-precision%29))
  (Utilities|Struct|SetmembersinS_Stat (Utilities|Array|Get(acopy) (Variables|Default|GetStat) (Stats|GetStatIndex Type)) NewValue)
  (Default|CallOnBaseValueChanged Type NewValue))

(fn GetDamage
  (return (Math|Conversions|ToFloat(Integer) (Math|Float|Truncate (* (.Value (Stats|GetStatValue "NewEnumerator4" false)) (select (<= (Math|Random|RandomFloatinRange 1.0 1e+02) (.Value (Stats|GetStatValue "NewEnumerator0" false))) (.Value (Stats|GetStatValue "NewEnumerator15" false)) 1.0))))))

(fn GetStatIndex
  (params (PlayerStats :type E_PlayerStats%20Enum :default "NewEnumerator0"))
  (for (_array_element _array_index) (Variables|Default|GetStat)
    (if (Utilities|Enum|Equal(Enum) (.PlayerStats (Utilities|Struct|BreakS_Stat _array_element)) PlayerStats)
      (return _array_index)))
  (return -1))

(fn GetStatValue
  (params (PlayerStats :type E_PlayerStats%20Enum :default "NewEnumerator0") (IncludeModifiers :type Boolean))
  (bind _output_get (LocalVariables|SetL_Index (Stats|GetStatIndex PlayerStats)))
  (if (>= _output_get 0)
    (return (Math|Float|SelectFloat (.BaseValue (Utilities|Struct|BreakS_Stat (Utilities|Array|Get(acopy) (Variables|Default|GetStat) (LocalVariables|GetL_Index)))) (+ (.BaseValue (Utilities|Struct|BreakS_Stat (Utilities|Array|Get(acopy) (Variables|Default|GetStat) (LocalVariables|GetL_Index)))) (.ModifiersValue (Utilities|Struct|BreakS_Stat (Utilities|Array|Get(acopy) (Variables|Default|GetStat) (LocalVariables|GetL_Index))))) IncludeModifiers) (.MaxValue (Utilities|Struct|BreakS_Stat (Utilities|Array|Get(acopy) (Variables|Default|GetStat) (LocalVariables|GetL_Index)))))))

(fn StatChanged
  (params (Value :type Float%20%28single-precision%29) (Type :type E_PlayerStats%20Enum :default "NewEnumerator0") (Removed? :type Boolean))
  (bind (_value _maxvalue) (Stats|GetStatValue Type false))
  (bind _returnvalue (- _value Value))
  (bind _returnvalue_2 (+ _value Value))
  (LocalVariables|SetL_MaxValue _maxvalue)
  (LocalVariables|SetL_Value _value)
  (if (!= Value 0.0)
    (if (>= _value 0.0)
      (if Removed?
        (Stats|ChangeStatBaseValue Type _returnvalue)
        (if (<= _returnvalue 0.0)
          (Stats|ChangeStatBaseValue Type 0.0)
          ;[1 1 1] -
          (Default|CallOnTakeDamage Value))
        (else
          (Stats|ChangeStatBaseValue Type _returnvalue_2)
          (if (>= _returnvalue_2 (LocalVariables|GetL_MaxValue))
            (Stats|ChangeStatBaseValue Type (LocalVariables|GetL_MaxValue))
            ;[1 1 1] +
            (Default|CallOnTakeDamage Value)))))))

(fn Atribut
  (params (Removed? :type Boolean) (Attribut :type E_PlayerStats%20Enum :default "NewEnumerator0") (ChangeParam-1 :type E_PlayerStats%20Enum :default "NewEnumerator0") (ChangeParam-1%20Value :type Float%20%28single-precision%29) (ChangeParam-2 :type E_PlayerStats%20Enum :default "NewEnumerator0") (ChangeParam-2%20Value :type Float%20%28single-precision%29) (ChangeParam-3 :type E_PlayerStats%20Enum :default "NewEnumerator0") (ChangeParam-3%20Value :type Float%20%28single-precision%29) (ChangeParam-4 :type E_PlayerStats%20Enum :default "NewEnumerator0") (String%204%20param :type Array%20of%20Strings) (Character%20lvl :type Float%20%28single-precision%29))
  (LocalVariables|SetL_Attribut1 ChangeParam-1%20Value)
  (CallFunction|StatChanged (LocalVariables|GetL_Attribut1) ChangeParam-1 Removed?)
  (CallFunction|StatChanged ChangeParam-2%20Value ChangeParam-2 Removed?)
  (CallFunction|StatChanged ChangeParam-3%20Value ChangeParam-3 Removed?)
  (CallFunction|StatChanged (Math|Conversions|ToFloat(Integer) (Utilities|Array|Get(acopy) String%204%20param (Math|Float|Ceil (.Value (Stats|GetStatValue Attribut false))))) ChangeParam-4 Removed?))

(fn AtributRazum
  (params (Removed? :type Boolean) (Attribut :type E_PlayerStats%20Enum :default "NewEnumerator0") (ChangeParam-1 :type E_PlayerStats%20Enum :default "NewEnumerator0") (String%201%20param :type Array%20of%20Strings) (ChangeParam-2 :type E_PlayerStats%20Enum :default "NewEnumerator0") (ChangeParam-2%20Value :type Float%20%28single-precision%29) (ChangeParam-3 :type E_PlayerStats%20Enum :default "NewEnumerator0") (ChangeParam-3%20Value :type Float%20%28single-precision%29) (ChangeParam-4 :type E_PlayerStats%20Enum :default "NewEnumerator0") (ChangeParam-4%20Value :type Float%20%28single-precision%29) (ChangeParam-5 :type E_PlayerStats%20Enum :default "NewEnumerator0") (ChangeParam-5%20Value :type Float%20%28single-precision%29) (ChangeParam-6 :type E_PlayerStats%20Enum :default "NewEnumerator0") (String%206%20param :type Array%20of%20Strings) (ChangeParam-7 :type E_PlayerStats%20Enum :default "NewEnumerator0") (ChangeParam-7%20Value :type Float%20%28single-precision%29) (Character%20lvl :type Float%20%28single-precision%29))
  (LocalVariables|SetL_Attribut2 ChangeParam-2%20Value)
  (CallFunction|StatChanged (Math|Conversions|ToFloat(Integer) (Utilities|Array|Get(acopy) String%201%20param (Math|Float|Ceil (.Value (Stats|GetStatValue Attribut false))))) ChangeParam-1 Removed?)
  (CallFunction|StatChanged (LocalVariables|GetL_Attribut2) ChangeParam-2 Removed?)
  (CallFunction|StatChanged ChangeParam-3%20Value ChangeParam-3 Removed?)
  (CallFunction|StatChanged ChangeParam-4%20Value ChangeParam-4 Removed?)
  (CallFunction|StatChanged ChangeParam-5%20Value ChangeParam-5 Removed?)
  (CallFunction|StatChanged (Math|Conversions|ToFloat(Integer) (Utilities|Array|Get(acopy) String%206%20param (Math|Float|Ceil (.Value (Stats|GetStatValue Attribut false))))) ChangeParam-6 Removed?)
  (CallFunction|StatChanged ChangeParam-7%20Value ChangeParam-7 Removed?))

(fn AtributLovkost
  (params (Removed? :type Boolean) (Attribut :type E_PlayerStats%20Enum :default "NewEnumerator0") (ChangeParam-1 :type E_PlayerStats%20Enum :default "NewEnumerator0") (ChangeParam-1%20Value :type Float%20%28single-precision%29) (ChangeParam-2 :type E_PlayerStats%20Enum :default "NewEnumerator0") (ChangeParam-2%20Value :type Float%20%28single-precision%29) (ChangeParam-3 :type E_PlayerStats%20Enum :default "NewEnumerator0") (String%203%20param :type Array%20of%20Strings) (ChangeParam-4 :type E_PlayerStats%20Enum :default "NewEnumerator0") (ChangeParam-4%20Value :type Float%20%28single-precision%29) (ChangeParam-5 :type E_PlayerStats%20Enum :default "NewEnumerator0") (ChangeParam-5%20Value :type Float%20%28single-precision%29) (ChangeParam-6 :type E_PlayerStats%20Enum :default "NewEnumerator0") (String%206%20param :type Array%20of%20Strings) (Character%20lvl :type Float%20%28single-precision%29))
  (CallFunction|StatChanged ChangeParam-1%20Value ChangeParam-1 Removed?)
  (CallFunction|StatChanged ChangeParam-2%20Value ChangeParam-2 Removed?)
  (CallFunction|StatChanged (Math|Conversions|ToFloat(Integer) (Utilities|Array|Get(acopy) String%203%20param (Math|Float|Ceil (.Value (Stats|GetStatValue Attribut false))))) ChangeParam-3 Removed?)
  (CallFunction|StatChanged ChangeParam-4%20Value ChangeParam-4 Removed?)
  (CallFunction|StatChanged ChangeParam-5%20Value ChangeParam-5 Removed?)
  (CallFunction|StatChanged (Math|Conversions|ToFloat(Integer) (Utilities|Array|Get(acopy) String%206%20param (Math|Float|Ceil (.Value (Stats|GetStatValue Attribut false))))) ChangeParam-6 Removed?))