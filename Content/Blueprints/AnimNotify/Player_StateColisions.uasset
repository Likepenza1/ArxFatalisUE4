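; Anim notify state, shown as Player_Collisions, that marks the attack hit window of the RPG player character during an animation.
; On begin it casts the mesh owner to BP_RPG_CharacterMain, sets AttackRelease, sets HitComponent to query-only collision and calls the character's weapon line trace.
; On end it clears AttackRelease but sets HitComponent to query-only again, so the notify never disables that collision.
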(fn GetNotifyName
  (return "Player_Collisions"))

(fn ReceivedNotifyBegin
  (params (MeshComp :type Skeletal%20Mesh%20Component%20Object%20Reference) (Animation :type Anim%20Sequence%20Base%20Object%20Reference) (TotalDuration :type Float%20%28single-precision%29))
  (bind _asbp_rpg_character_main (Utilities|Casting|CastToBP_RPG_CharacterMain (Components|GetOwner MeshComp)))
  (Variables|/Game/RPGCharacterCreator/Characters/BP_RPG_CharacterMain.BP_RPG_CharacterMain_C|SetAttackRelease? _asbp_rpg_character_main true)
  (Collision|SetCollisionEnabled (Variables|/Game/RPGCharacterCreator/Characters/BP_RPG_CharacterMain.BP_RPG_CharacterMain_C|GetHit%20Component _asbp_rpg_character_main) "QueryOnly")
  (Default|LineTraceWeaponColisions _asbp_rpg_character_main)
  (return false))

(fn ReceivedNotifyEnd
  (params (MeshComp :type Skeletal%20Mesh%20Component%20Object%20Reference) (Animation :type Anim%20Sequence%20Base%20Object%20Reference))
  (bind _asbp_rpg_character_main (Utilities|Casting|CastToBP_RPG_CharacterMain (Components|GetOwner MeshComp)))
  (Variables|/Game/RPGCharacterCreator/Characters/BP_RPG_CharacterMain.BP_RPG_CharacterMain_C|SetAttackRelease? _asbp_rpg_character_main false)
  (Collision|SetCollisionEnabled (Variables|/Game/RPGCharacterCreator/Characters/BP_RPG_CharacterMain.BP_RPG_CharacterMain_C|GetHit%20Component _asbp_rpg_character_main) "QueryOnly")
  (return false))