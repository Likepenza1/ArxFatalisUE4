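; Animation notify state, shown as WeaponHIT_Collisions, that opens a hit-detection window during a monster's animation.
; On begin it casts the mesh owner to Monster_NBC and sets its CapsuleHit collision to query-only.
; On end it disables that collision again, so the capsule follows the notify's span on the animation timeline.
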(fn GetNotifyName
  (return "WeaponHIT_Collisions"))

(fn ReceivedNotifyBegin
  (params (MeshComp :type Skeletal%20Mesh%20Component%20Object%20Reference) (Animation :type Anim%20Sequence%20Base%20Object%20Reference) (TotalDuration :type Float%20%28single-precision%29))
  (bind _asmonster_nbc (Utilities|Casting|CastToMonster_NBC (Components|GetOwner MeshComp)))
  (Utilities|IsValid (Variables|/Game/MonsterAi_Kit/Monster_NBC.Monster_NBC_C|GetCapsuleHit _asmonster_nbc)
    (:Is%20Valid
      (Collision|SetCollisionEnabled (Variables|/Game/MonsterAi_Kit/Monster_NBC.Monster_NBC_C|GetCapsuleHit _asmonster_nbc) "QueryOnly"))
    (:Is%20Not%20Valid
      _))
  (return false))

(fn ReceivedNotifyEnd
  (params (MeshComp :type Skeletal%20Mesh%20Component%20Object%20Reference) (Animation :type Anim%20Sequence%20Base%20Object%20Reference))
  (bind _asmonster_nbc (Utilities|Casting|CastToMonster_NBC (Components|GetOwner MeshComp)))
  (Utilities|IsValid (Variables|/Game/MonsterAi_Kit/Monster_NBC.Monster_NBC_C|GetCapsuleHit _asmonster_nbc)
    (:Is%20Valid
      (Collision|SetCollisionEnabled (Variables|/Game/MonsterAi_Kit/Monster_NBC.Monster_NBC_C|GetCapsuleHit _asmonster_nbc) "NoCollision"))
    (:Is%20Not%20Valid
      _))
  (return false))