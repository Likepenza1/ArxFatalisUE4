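; Interactable, lockable swinging door, configurable as a single metal, single wood or double door by toggling mesh visibility and collision.
; When locked, interaction looks up KeyItemID in the item data table and unlocks if the player's inventory holds it.
; Otherwise it toggles DoorState, playing sounds and timeline-driven rotations behind a Moving guard.
; Save functions store lock and open state; a separate UpdateDoor event snaps rotation from them.
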(event Custom|Used
  (bind _returnvalue (Transformation|GetActorLocation))
  (bind _returnvalue_2 (Transformation|GetActorLocation))
  (bind _returnvalue_3 (Transformation|GetActorLocation))
  (if (Variables|Default|GetClosedDor)
    (Utilities|CheckKey
      (:Key%20Found
        (Audio|PlaySoundatLocation "/Game/Blueprints/DOOR/L1/Door_unlock.Door_unlock" _returnvalue_3 "0, 0, 0" 1.0 1.0 0.0 0 0 0)
        (Variables|Default|SetClosedDor false))
      (:Key%20NOT%20Found
        (Audio|PlaySoundatLocation "/Game/SFX/Player_CLOSEDDOOP/player_locked.player_locked" _returnvalue_3 "0, 0, 0" 1.0 1.0 0.0 0 0 0)
        (Audio|PlaySoundatLocation "/Game/SFX/Player_CLOSEDDOOP/door_wrong_key.door_wrong_key" _returnvalue_3 "0, 0, 0" 1.0 1.0 0.0 0 0 0)))
    (elif (not (Variables|Default|GetDoobleDoor))
      (if (not (Variables|Default|GetMoving))
        (Variables|Default|SetMoving true)
        (switch int (Variables|Default|GetDoorState)
          (:0
            (Variables|Default|SetDoorState 1)
            (if (Variables|Default|GetwoodDoorLight)
              (Audio|PlaySoundatLocation "/Game/Blueprints/DOOR/L1/door_wood_open.door_wood_open" _returnvalue "0, 0, 0" 1.0 1.0 0.0 0 0 0)
              (bind _leverr (Timeline|Timeline_3 PlayFromStart)
                (:Update
                  (Transformation|SetRelativeRotation (Variables|Default|Gete) (Math|Rotator|MakeRotator 0.0 0.0 (+ _leverr (.yaw (Variables|Default|GetInitRot)))) false false)
                  (Utilities|FlowControl|Delay 1.0)
                  (Variables|Default|SetMoving false)))
              (else
                (Audio|PlaySoundatLocation "/Game/Blueprints/DOOR/L1/door_metal_open.door_metal_open" _returnvalue "0, 0, 0" 1.0 1.0 0.0 0 0 0)
                (bind _leverr_2 (Timeline|Timeline_0 PlayFromStart)
                  (:Update
                    (Transformation|SetRelativeRotation (Variables|Default|Gete) (Math|Rotator|MakeRotator 0.0 0.0 (+ _leverr_2 (.yaw (Variables|Default|GetInitRot)))) false false)
                    (Utilities|FlowControl|Delay 1.2)
                    (Variables|Default|SetMoving false))))))
          (:1
            (Variables|Default|SetDoorState 0)
            (if (Variables|Default|GetwoodDoorLight)
              (Audio|PlaySoundatLocation "/Game/Blueprints/DOOR/L1/door_wood_close.door_wood_close" _returnvalue "0, 0, 0" 1.0 1.0 0.0 0 0 0)
              (Timeline|Timeline_3 ReverseFromEnd)
              (else
                (Audio|PlaySoundatLocation "/Game/Blueprints/DOOR/L1/door_metal_close.door_metal_close" _returnvalue "0, 0, 0" 1.0 1.0 0.0 0 0 0)
                (Timeline|Timeline_0 ReverseFromEnd))))))
      (elif (not (Variables|Default|GetMoving))
        (Variables|Default|SetMoving true)
        (switch int (Variables|Default|GetDoorState)
          (:0
            (Variables|Default|SetDoorState 1)
            (Audio|PlaySoundatLocation "/Game/Blueprints/DOOR/L1/door_metal_open.door_metal_open" _returnvalue_2 "0, 0, 0" 1.0 1.0 0.0 0 0 0)
            (Utilities|FlowControl|Sequence
              (:then_0
                (bind _leverr_3 (Timeline|Timeline_1 PlayFromStart)
                  (:Update
                    (Transformation|SetRelativeRotation (Variables|Default|Gete1) (Math|Rotator|MakeRotator 0.0 0.0 (+ _leverr_3 (.yaw (Variables|Default|GetInitRot)))) false false)
                    (Utilities|FlowControl|Delay 1.2 :!label _label)
                    (Variables|Default|SetMoving false))))
              (:then_1
                (bind _leverr_4 (Timeline|Timeline_2 PlayFromStart)
                  (:Update
                    (Transformation|SetRelativeRotation (Variables|Default|Gete2) (Math|Rotator|MakeRotator 0.0 0.0 (+ _leverr_4 (.yaw (Variables|Default|GetInitRot_1)))) false false)
                    (goto _label))))))
          (:1
            (Variables|Default|SetDoorState 0)
            (Audio|PlaySoundatLocation "/Game/Blueprints/DOOR/L1/door_dbl_metal_close.door_dbl_metal_close" _returnvalue_2 "0, 0, 0" 1.0 1.0 0.0 0 0 0)
            (Utilities|FlowControl|Sequence
              (:then_0
                (Timeline|Timeline_1 ReverseFromEnd))
              (:then_1
                (Timeline|Timeline_2 ReverseFromEnd)))))))))

(event Custom|UpdateDoor
  (bind _e2 (Variables|Default|Gete2))
  (bind _e (Variables|Default|Gete))
  (bind _e1 (Variables|Default|Gete1))
  (if (Variables|Default|GetDoobleDoor)
    (if (== (Variables|Default|GetDoorState) 1)
      (Transformation|SetRelativeRotation _e1 (Math|Rotator|MakeRotator 0.0 0.0 -9e+01) false false)
      (Transformation|SetRelativeRotation _e2 (Math|Rotator|MakeRotator 0.0 0.0 9e+01) false false)
      (elif (Variables|Default|GetClosedDor)
        (Transformation|SetRelativeRotation _e1 (Math|Rotator|MakeRotator 0.0 0.0 0.0) false false)
        (Transformation|SetRelativeRotation _e2 (Math|Rotator|MakeRotator 0.0 0.0 0.0) false false)))
    (elif (== (Variables|Default|GetDoorState) 1)
      (Transformation|SetRelativeRotation _e (Math|Rotator|MakeRotator 0.0 0.0 -9e+01) false false)
      (elif (Variables|Default|GetClosedDor)
        (Transformation|SetRelativeRotation _e (Math|Rotator|MakeRotator 0.0 0.0 0.0) false false)))))

(event EventBPILoadDone
  ;[1 1 1] Save/Load
  (CallFunction|LoadDone))

(event EventBeginPlay
  (if (Variables|Default|GetDoobleDoor)
    (Utilities|FlowControl|Sequence
      (:then_0
        (Utilities|FlowControl|Sequence
          (:then_0
            (Collision|SetCollisionEnabled (Variables|Default|GetDoor2) "QueryAndPhysics"))
          (:then_1
            (Collision|SetCollisionEnabled (Variables|Default|GetDoor) "PhysicsOnly"))))
      (:then_1
        (Rendering|SetVisibility (Variables|Default|GetDoor3) true false)
        (Rendering|SetVisibility (Variables|Default|GetDoor) false false)))
    (elif (Variables|Default|GetwoodDoorLight)
      (Utilities|FlowControl|Sequence
        (:then_0
          (Collision|SetCollisionEnabled (Variables|Default|GetDoor2) "PhysicsOnly"))
        (:then_1
          (Collision|SetCollisionEnabled (Variables|Default|GetDoor) "QueryAndPhysics"))
        (:then_2
          (Rendering|SetVisibility (Variables|Default|GetDoor3) false false)
          (Rendering|SetVisibility (Variables|Default|GetWoodDoor) true false)))
      (else
        (Utilities|FlowControl|Sequence
          (:then_0
            (Utilities|FlowControl|Sequence
              (:then_0
                (Collision|SetCollisionEnabled (Variables|Default|GetDoor2) "PhysicsOnly"))
              (:then_1
                (Collision|SetCollisionEnabled (Variables|Default|GetDoor) "QueryAndPhysics"))))
          (:then_1
            (Rendering|SetVisibility (Variables|Default|GetDoor3) false false)
            (Rendering|SetVisibility (Variables|Default|GetDoor) true false)))))))

(event EventBPILoadState
  (params (SaveSlot :type S%20Save%20Actor%20Structure))
  ;[1 1 1] Save/Load
  (CallFunction|LoadState SaveSlot))

(event EventBInteraction
  (CallFunction|Used))

(fn ConstructionScript
  (if (Variables|Default|GetDoobleDoor)
    (Rendering|SetVisibility (Variables|Default|GetDoor3) true false)
    (Rendering|SetVisibility (Variables|Default|GetDoor) false false)
    (elif (Variables|Default|GetwoodDoorLight)
      (Rendering|SetVisibility (Variables|Default|GetDoor3) false false)
      (Rendering|SetVisibility (Variables|Default|GetWoodDoor) true false)
      (else
        (Rendering|SetVisibility (Variables|Default|GetDoor3) false false)
        (Rendering|SetVisibility (Variables|Default|GetDoor) true false)))))

(fn SaveState
  (params (Save%20Data%20Add%20Add :type S%20Save%20Actor%20Add%20Structure))
  (return (Utilities|Struct|MakeS_SaveActor "0.000000,0.000000,0.000000|0.000000,0.000000,0.000000|1.000000,1.000000,1.000000" (Utilities|GetClass self) false (Variables|Default|GetClosedDor) "(BoolArray_2_0C11053C44F85D099D01009D36B474A2=)" self 0 "(Items_4_E2E953BB4A67DC946206EF9D2DA87881=())" (Variables|Default|GetDoorState) 0.0)))

(fn LoadState
  (params (SaveDataAdd :type S%20Save%20Actor%20Structure))
  (Variables|Default|SetLoaded true)
  (Variables|Default|SetClosedDor (.ison SaveDataAdd))
  (Variables|Default|SetDoorState (.integer SaveDataAdd)))

(fn LoadDone
  (if (not (Variables|Default|GetLoaded))
    (return)))

(fn BPISaveState
  (return (Utilities|Struct|MakeS_SaveActor "0.000000,0.000000,0.000000|0.000000,0.000000,0.000000|1.000000,1.000000,1.000000" 0 false (Variables|Default|GetClosedDor) (Utilities|Struct|MakeS_SaveActorAdd 0) 0 0 "(Items_4_E2E953BB4A67DC946206EF9D2DA87881=())" (Variables|Default|GetDoorState))))

(fn ICanbeInteracted
  (return true))

(fn IEndInteraction
  (params (InteractingCharacter :type Character%20Object%20Reference))
  (return false))

(fn IGetInteractionText
  (return "" ""))

(fn IGetInventoryItems
  (return 0))

(fn IInteraction
  (params (InteractingCharacter :type Character%20Object%20Reference))
  (return "Железная дверь" true))

(fn ISetInventoryItems
  (params (Items :type Map%20of%20ST%20Item%20Slot%20Params%20Structures%20to%20Structs))
  (return false))