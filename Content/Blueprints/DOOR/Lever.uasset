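; Interactable lever actor that opens and closes a tagged GateGoblins gate, found on BeginPlay.
; BInteraction runs Used, which toggles DoorState, notifies the gate and plays or reverses a timeline that pitches the lever mesh.
; UpdateLever and LeverPos snap the lever to either end, with UpdateLever also pushing DoorState to the gate.
; Save/load stores only the Moving flag; LoadDone applies nothing, and most interaction interface functions are stubs.
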(event Custom|Used
  (bind _gate (Variables|Default|GetGate))
  (switch int (Variables|Default|GetDoorState)
    (:0
      (Variables|Default|SetDoorState 1)
      (Variables|Default|SetMoving true)
      (Default|GateUsed _gate true)
      (bind _leverr (Timeline|leverR PlayFromStart)
        (:Update
          (Transformation|SetRelativeRotation (Variables|Default|GetLever) (Math|Rotator|MakeRotator 0.0 (+ _leverr (.pitch (Variables|Default|GetInitRot))) 0.0) false false))))
    (:1
      (Variables|Default|SetDoorState 0)
      (Variables|Default|SetMoving false)
      (Default|GateUsed _gate false)
      (Timeline|leverR ReverseFromEnd))))

(event Custom|LeverPos
  (params (Condition :type Boolean))
  (Transformation|SetRelativeRotation (Variables|Default|GetLever) (Math|Rotator|SelectRotator (Math|Rotator|MakeRotator 0.0 (+ 4e+01 (.pitch (Variables|Default|GetInitRot))) 0.0) (Math|Rotator|MakeRotator 0.0 (- -29.0 (.pitch (Variables|Default|GetInitRot))) 0.0) Condition) false false))

(event Custom|UpdateLever
  (bind _doorstate (Variables|Default|GetDoorState))
  (Default|StatusGate (Variables|Default|GetGate) _doorstate)
  (if (== _doorstate 1)
    (Transformation|SetRelativeRotation (Variables|Default|GetLever) "40.000000, 0, 0" false false)
    (else
      (Transformation|SetRelativeRotation (Variables|Default|GetLever) "-29.000000, 0, 0" false false))))

(event EventBPILoadDone
  ;[1 1 1] Save/Load
  (CallFunction|LoadDone))

(event EventBeginPlay
  (bind _outactors (Actor|GetAllActorsOfClasswithTag "/Game/Blueprints/DOOR/GateGoblins.GateGoblins_C" (Variables|Default|GetTagGate)))
  (Variables|Default|SetGate (Utilities|Array|Get(acopy) _outactors)))

(event EventBPILoadState
  (params (SaveSlot :type S%20Save%20Actor%20Structure))
  ;[1 1 1] Save/Load
  (CallFunction|LoadState SaveSlot))

(event EventBInteraction
  (CallFunction|Used))

(fn ConstructionScript
  (bind _returnvalue (Transformation|GetActorRotation))
  (Transformation|SetActorRotation _returnvalue)
  (Variables|Default|SetInitRot _returnvalue))

(fn SaveState
  (params (Save%20Data%20Add%20Add :type S%20Save%20Actor%20Add%20Structure))
  (return (Utilities|Struct|MakeS_SaveActor "0.000000,0.000000,0.000000|0.000000,0.000000,0.000000|1.000000,1.000000,1.000000" (Utilities|GetClass self) false (Variables|Default|GetMoving) "(BoolArray_2_0C11053C44F85D099D01009D36B474A2=)" self 0 "(Items_4_E2E953BB4A67DC946206EF9D2DA87881=())" 0 0.0)))

(fn LoadState
  (params (SaveDataAdd :type S%20Save%20Actor%20Structure))
  (Variables|Default|SetLoaded true)
  (Variables|Default|SetMoving (.ison SaveDataAdd)))

(fn LoadDone
  (if (not (Variables|Default|GetLoaded))
    (return)))

(fn BPISaveState
  (return (Utilities|Struct|MakeS_SaveActor "0.000000,0.000000,0.000000|0.000000,0.000000,0.000000|1.000000,1.000000,1.000000" 0 false (Variables|Default|GetMoving))))

(fn ICanbeInteracted
  (return true))

(fn IEndInteraction
  (params (InteractingCharacter :type Character%20Object%20Reference))
  (return false))

(fn IGetInteractionText
  (return "" ""))

(fn IGetInventoryItems
  (return 0))

(fn IInteraction
  (params (InteractingCharacter :type Character%20Object%20Reference))
  (return "" true))

(fn ISetInventoryItems
  (params (Items :type Map%20of%20ST%20Item%20Slot%20Params%20Structures%20to%20Structs))
  (return false))