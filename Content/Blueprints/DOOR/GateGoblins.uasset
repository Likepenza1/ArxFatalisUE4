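; GateGoblins is a portcullis gate Blueprint that raises and lowers with sound.
; GateUsed drives it: opening runs once behind a DoOnce, playing a timeline that lifts the Scene component and disables Gate collision.
; Closing resets the DoOnce, plays the close sound and runs a second timeline that moves the Scene and re-enables collision.
; StatusGate snaps the Scene straight to the raised or default height from a status value.
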(event Custom|GateUsed
  (params (Up? :type Boolean))
  (bind _returnvalue (Transformation|GetActorLocation))
  (if Up?
    (Utilities|FlowControl|DoOnce false :!label _label
      (:Completed
        (Audio|PlaySoundatLocation "/Game/SFX/gateOpen/porticullis_open.porticullis_open" _returnvalue "0, 0, 0" 1.0 1.0 0.0 0 0 0)
        (bind _newtrack_0 (Timeline|GATE_UP PlayFromStart)
          (:Update
            (Transformation|SetRelativeLocation (Variables|Default|GetScene) (Math|Vector|MakeVector 0.0 0.0 _newtrack_0) false false)
            (Collision|SetCollisionEnabled (Variables|Default|Getgate) "NoCollision")))))
    (else
      (Utilities|FlowControl|Sequence
        (:then_0
          (goto _label Reset))
        (:then_1
          (Audio|PlaySoundatLocation "/Game/SFX/gateOpen/porticullis_close.porticullis_close" _returnvalue "0, 0, 0" 1.0 1.0 0.0 0 0 0)
          (bind _newtrack_0_2 (Timeline|GateDown PlayFromStart)
            (:Update
              (Transformation|SetRelativeLocation (Variables|Default|GetScene) (Math|Vector|MakeVector 0.0 0.0 _newtrack_0_2) false false)
              (Collision|SetCollisionEnabled (Variables|Default|Getgate) "QueryAndPhysics"))))))))

(event Custom|StatusGate
  (params (NewParam :type Integer))
  (bind _scene (Variables|Default|GetScene))
  (if (== NewParam 1)
    (Transformation|SetRelativeLocation _scene (Math|Vector|MakeVector 0.0 0.0 212.0) false false)
    (else
      (Transformation|SetRelativeLocation _scene (Math|Vector|MakeVector 0.0 0.0 0.0) false false))))

(fn ConstructionScript)