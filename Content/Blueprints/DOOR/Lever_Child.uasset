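; Lever_Child is a child lever Blueprint, filed with the door assets, that adds save and load support for the lever's on/off state.
; SaveState passes the Moving flag to the parent as extra save data, and LoadState restores it from IsOn.
; UpdateLoad maps Moving to a DoorState of 1 or 0, running on load and again in LoadDone, and LoadState then calls UpdateLever to refresh the lever.
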(event EventBeginPlay
  (|CallParentFunction))

(event Collision|EventActorBeginOverlap
  (params (OtherActor :type Actor%20Object%20Reference)))

(event EventTick
  (params (DeltaSeconds :type Float%20%28single-precision%29))
  (|CallParentFunction DeltaSeconds) ; This node is disabled and will not be called.\nDrag off pins to build functionality.
)

(fn ConstructionScript
  (|CallParentFunction))

(fn LoadState
  (params (SaveDataAdd :type S%20Save%20Actor%20Structure))
  (|CallParentFunction SaveDataAdd)
  (Variables|Default|SetMoving (.IsOn (Utilities|Struct|BreakS_SaveActor SaveDataAdd)))
  (CallFunction|UpdateLoad)
  (CallFunction|UpdateLever))

(fn SaveState
  (params (Save%20Data%20Add%20Add :type S%20Save%20Actor%20Add%20Structure))
  (bind _save_data (|CallParentFunction (Utilities|Struct|MakeS_SaveActorAdd (Utilities|Array|MakeArray (Variables|Default|GetMoving)))))
  (return _save_data))

(fn LoadDone
  (|CallParentFunction)
  (CallFunction|UpdateLoad))

(fn UpdateLoad
  (if (Variables|Default|GetMoving)
    (Variables|Default|SetDoorState 1)
    (else
      (Variables|Default|SetDoorState 0))))