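; Storage is an interactable container Blueprint with a configurable mesh that opens an inventory screen for the player.
; It creates an inventory widget bound to its InventoryComponent at BeginPlay and supplies its name through Informations.
; Interactions toggles that widget alongside the player's inventory, showing the cursor on open and ignoring input during drag and drop.
; When the player leaves the Box trigger, both inventories hide automatically.
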(event OnComponentEndOverlap(Box)
  (params (OverlappedComponent :type Primitive%20Component%20Object%20Reference) (OtherActor :type Actor%20Object%20Reference) (OtherComp :type Primitive%20Component%20Object%20Reference) (OtherBodyIndex :type Integer))
  (if (== OtherActor (CallFunction|--GetPlayerCharacter))
    (if (UserInterface|Viewport|IsinViewport (Variables|Default|GetStorage))
      (Default|AnimationInventoryHide (Variables|Default|GetStorage))
      (Default|-HideInv (CallFunction|--GetPlayerCharacter)))))

(event EventBeginPlay
  (bind _returnvalue (UserInterface|CreateWidget "/Game/Blueprints/widget/Storage/Inventory_Widget_storage.Inventory_Widget_storage_C" (CallFunction|--PlayerController) (Variables|Default|GetInventoryComponent) 1.3e+02))
  (Variables|Default|SetStorage _returnvalue))

(event EventInteractions
  (bind _newparam (CallFunction|--PlayerController))
  (bind _storage (Variables|Default|GetStorage))
  (if (not (Class|WidgetBlueprintLibrary|IsDragDropping))
    (if (UserInterface|Viewport|IsinViewport (Variables|Default|GetStorage))
      (Default|AnimationInventoryHide _storage)
      (Default|-HideInv (CallFunction|--GetPlayerCharacter))
      (else
        (UserInterface|Viewport|AddtoViewport _storage 2)
        (Input|SetInputModeGameandUI _newparam (Variables|Default|GetStorage) "DoNotLock" false)
        (Variables|/Script/Engine.PlayerController|SetbShowMouseCursor _newparam true)
        (Default|AnimationInventoryVisible (Variables|Default|GetStorage))
        (Default|-VisibleInv (CallFunction|--GetPlayerCharacter))))))

(fn ConstructionScript
  (Components|StaticMesh|SetStaticMesh (Variables|Default|GetStaticMesh) (Variables|Default|GetNew%20Mesh)))

(fn Informations
  (return (Variables|Default|GetName) true))