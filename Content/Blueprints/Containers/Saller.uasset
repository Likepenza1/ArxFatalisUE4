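; Saller is a vendor container Blueprint that offers items for sale through an inventory screen.
; On BeginPlay it creates a seller inventory widget bound to its InventoryComponent and stocks it with hardcoded, priced BP_ItemObjects for leather legs and a club.
; Interacting toggles that widget and the player's inventory together unless a drag is active, enabling cursor and UI input on opening.
; When the player leaves the Box overlap, both inventories hide.
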(event OnComponentEndOverlap(Box)
  (params (OverlappedComponent :type Primitive%20Component%20Object%20Reference) (OtherActor :type Actor%20Object%20Reference) (OtherComp :type Primitive%20Component%20Object%20Reference) (OtherBodyIndex :type Integer))
  (if (== OtherActor (CallFunction|--GetPlayerCharacter))
    (if (UserInterface|Viewport|IsinViewport (Variables|Default|GetStorage))
      (Default|AnimationInventoryHide (Variables|Default|GetStorage))
      (Default|-HideInv (CallFunction|--GetPlayerCharacter)))))

(event EventBeginPlay
  (bind _returnvalue (UserInterface|CreateWidget "/Game/Blueprints/widget/Saller/Inventory_Widget_salle.Inventory_Widget_salle_C" (CallFunction|--PlayerController) (Variables|Default|GetInventoryComponent) 1.3e+02))
  (Variables|Default|SetStorage _returnvalue)
  (bind _returnvalue_2 (Game|ConstructObjectfromClass "/Game/Blueprints/ITEMS/BP_ItemObject.BP_ItemObject_C" "/Game/Blueprints/ITEMS/BP_LeatherLegs.BP_LeatherLegs" (Utilities|Struct|MakeIntPoint 2 3) "/Game/Blueprints/ITEMS/itemsIco/M_IconLweggingLeather.M_IconLweggingLeather" "/Game/Blueprints/ITEMS/itemsIco/M_IconLweggingLeather_R.M_IconLweggingLeather_R" "/Game/Blueprints/ITEMS/BP_LeatherLegs.BP_LeatherLegs_C" true 75))
  (Default|TryAddItem (Variables|Default|GetInventoryComponent) _returnvalue_2)
  (bind _returnvalue_3 (Game|ConstructObjectfromClass "/Game/Blueprints/ITEMS/BP_ItemObject.BP_ItemObject_C" "/Game/Blueprints/ITEMS/BP_Club.BP_Club" (Utilities|Struct|MakeIntPoint 1 2) "/Game/Blueprints/ITEMS/itemsIco/M_IconClub.M_IconClub" "/Game/Blueprints/ITEMS/itemsIco/M_IconClub_R.M_IconClub_R" "/Game/Blueprints/ITEMS/BP_Club.BP_Club_C" true 15))
  (Default|TryAddItem (Variables|Default|GetInventoryComponent) _returnvalue_3))

(event EventInteractions
  (bind _newparam (CallFunction|--PlayerController))
  (bind _storage (Variables|Default|GetStorage))
  (if (not (Class|WidgetBlueprintLibrary|IsDragDropping))
    (if (UserInterface|Viewport|IsinViewport (Variables|Default|GetStorage))
      (Default|AnimationInventoryHide _storage)
      (Default|-HideInv (CallFunction|--GetPlayerCharacter))
      (else
        (UserInterface|Viewport|AddtoViewport _storage 2)
        (Input|SetInputModeGameandUI _newparam (Variables|Default|GetStorage) "DoNotLock" false)
        (Variables|/Script/Engine.PlayerController|SetbShowMouseCursor _newparam true)
        (Default|AnimationInventoryVisible (Variables|Default|GetStorage))
        (Default|-VisibleInv (CallFunction|--GetPlayerCharacter))))))

(fn ConstructionScript)

(fn Informations
  (return (Variables|Default|GetName) true))