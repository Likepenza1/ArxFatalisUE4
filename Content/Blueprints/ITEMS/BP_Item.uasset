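; BP_Item is a world item actor that wraps an ItemObject and can be picked up or used through the player's InventoryComponent.
; BeginPlay fills a missing ItemObject from GetDefaultItemObject, which is empty here.
; Pickup tries to add the item, while Interactions marks it used and calls UseItem; either destroys the actor on success.
; Informations returns the item's name, and the equip logic is left disconnected.
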(event EventBeginPlay
  (if (not (Utilities|IsValid (Variables|Private|GetItemObject)))
    (bind _itemobject (Private|GetDefaultItemObject))
    (Variables|Private|SetItemObject _itemobject)))

(event EventPickup
  (bind _added (Default|TryAddItem (Variables|/Game/Blueprints/BP_AmShegar.BP_AmShegar_C|GetInventoryComponent (CallFunction|--GetPlayerCharacter)) (Variables|Private|GetItemObject)))
  (if _added
    (Actor|DestroyActor)))

(event EventInteractions
  (bind _itemobject (Variables|Private|GetItemObject))
  (Variables|/Game/Blueprints/ITEMS/BP_ItemObject.BP_ItemObject_C|SetUSED _itemobject true)
  (Development|PrintString (Utilities|GetDisplayName _itemobject))
  (bind _used (Default|UseItem (Variables|/Game/Blueprints/BP_AmShegar.BP_AmShegar_C|GetInventoryComponent (CallFunction|--GetPlayerCharacter)) (Variables|Private|GetItemObject)))
  (if _used
    (Actor|DestroyActor)))

(event EventTick
  (params (DeltaSeconds :type Float%20%28single-precision%29)))

(fn ConstructionScript)

(fn GetDefaultItemObject
  (return 0))

(fn Informations
  (return (Variables|Default|GetName) true))