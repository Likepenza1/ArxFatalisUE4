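; BP_InteractWorld is an interactable world actor with save/load support, apparently a base, with mostly stub interaction interface functions.
; Interaction always succeeds, returning the name "Решётка" (grate) with empty prompt text and no inventory handling.
; Loading restores an integer State and teleports the actor to its saved transform.
; SaveState records both, while BPI_SaveState stores only the transform; LoadDone is effectively empty.
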(event EventBPILoadDone
  ;[1 1 1] Save/Load
  (CallFunction|LoadDone))

(event Collision|EventActorBeginOverlap
  (params (OtherActor :type Actor%20Object%20Reference)))

(event EventBPILoadState
  (params (SaveSlot :type S%20Save%20Actor%20Structure))
  ;[1 1 1] Save/Load
  (CallFunction|LoadState SaveSlot))

(event EventBeginPlay)

(fn ConstructionScript)

(fn DestroySelf
  (Actor|DestroyActor))

(fn LoadDone
  (if (not (Variables|Default|GetLoaded))
    (return)))

(fn LoadState
  (params (SaveDataAdd :type S%20Save%20Actor%20Structure))
  (Variables|Default|SetLoaded true)
  (Variables|Default|SetState (.integer SaveDataAdd))
  (Transformation|SetActorTransform self (.position SaveDataAdd) false true))

(fn SaveState
  (params (Save%20Data%20Add%20Add :type S%20Save%20Actor%20Add%20Structure))
  (return (Utilities|Struct|MakeS_SaveActor (Transformation|GetActorTransform) (Utilities|GetClass self) false false "(BoolArray_2_0C11053C44F85D099D01009D36B474A2=)" self 0 "(Items_4_E2E953BB4A67DC946206EF9D2DA87881=())" (Variables|Default|GetState) 0.0)))

(fn BPISaveState
  (return (Utilities|Struct|MakeS_SaveActor (Transformation|GetActorTransform))))

(fn ICanbeInteracted
  (return true))

(fn IEndInteraction
  (params (InteractingCharacter :type Character%20Object%20Reference))
  (return true))

(fn IGetInteractionText
  (return "" ""))

(fn IGetInventoryItems
  (return 0))

(fn IInteraction
  (params (InteractingCharacter :type Character%20Object%20Reference))
  (return "Решётка" true false))

(fn ISetInventoryItems
  (params (Items :type Map%20of%20ST%20Item%20Slot%20Params%20Structures%20to%20Structs))
  (return false))