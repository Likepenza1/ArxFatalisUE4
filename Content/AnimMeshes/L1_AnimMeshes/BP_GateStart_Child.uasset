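; Interactive start gate, a child Blueprint that opens once on interaction and persists its state through the save system.
; Interaction swaps the static mesh SM1 for two animated skeletal meshes, removes its collision, plays sounds and sets State to 1.
; Player overlap with Box1 triggers a one-time custom-depth highlight and sound while unused, cleared on exit.
; Loading restores transform and State, then UpdateStatus shows either the idle skeletal meshes or the solid static mesh.
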(event OnComponentBeginOverlap(Box1)
  (params (OverlappedComponent :type Primitive%20Component%20Object%20Reference) (OtherActor :type Actor%20Object%20Reference) (OtherComp :type Primitive%20Component%20Object%20Reference) (OtherBodyIndex :type Integer) (bFromSweep :type Boolean) (SweepResult :type Hit%20Result%20Structure%20%28by%20ref%29))
  (if (== (CallFunction|--GetPlayerCharacter) OtherActor)
    (if (== (Variables|Default|GetState) 0)
      (Utilities|FlowControl|DoOnce false
        (:Completed
          (Rendering|SetRenderCustomDepth (Variables|Default|GetSM1) true)
          (Audio|PlaySoundatLocation "/Game/SFX/System/system2.system2" (Transformation|GetActorLocation) "0, 0, 0" 1.0 1.0 0.0 0 0 0))))))

(event OnComponentEndOverlap(Box1)
  (params (OverlappedComponent :type Primitive%20Component%20Object%20Reference) (OtherActor :type Actor%20Object%20Reference) (OtherComp :type Primitive%20Component%20Object%20Reference) (OtherBodyIndex :type Integer))
  (if (== (CallFunction|--GetPlayerCharacter) OtherActor)
    (Rendering|SetRenderCustomDepth (Variables|Default|GetSM1) false)))

(event EventBeginPlay
  (|CallParentFunction) ; This node is disabled and will not be called.\nDrag off pins to build functionality.
)

(event Collision|EventActorBeginOverlap
  (params (OtherActor :type Actor%20Object%20Reference))
  (|CallParentFunction OtherActor) ; This node is disabled and will not be called.\nDrag off pins to build functionality.
)

(event EventTick
  (params (DeltaSeconds :type Float%20%28single-precision%29))
  (|CallParentFunction DeltaSeconds) ; This node is disabled and will not be called.\nDrag off pins to build functionality.
)

(event EventBInteraction
  (bind _returnvalue (Transformation|GetActorLocation))
  (bind _sm1 (Variables|Default|GetSM1))
  (Rendering|SetVisibility (Variables|Default|GetSK2) true false)
  (Components|Animation|PlayAnimation (Variables|Default|GetSK1) "/Game/AnimMeshes/L1_AnimMeshes/AnimGate.AnimGate" false)
  (Rendering|SetVisibility _sm1 false false)
  (Collision|SetCollisionEnabled _sm1 "NoCollision")
  (Audio|PlaySoundatLocation "/Game/SFX/gateOpen/porticulis_Twist.porticulis_Twist" _returnvalue "0, 0, 0" 1.0 1.0 0.0 0 0 0)
  (Audio|PlaySoundatLocation "/Game/NPC/KultarNPC/Song/Kultar_encourage_Cue.Kultar_encourage_Cue" _returnvalue "0, 0, 0" 1.0 1.0 0.0 0 0 0)
  (Variables|Default|SetState 1))

(fn ConstructionScript
  (|CallParentFunction))

(fn BPISaveState
  (return (Utilities|Struct|MakeS_SaveActor (Transformation|GetActorTransform) 0 false false (Utilities|Struct|MakeS_SaveActorAdd 0) 0 0 "(Items_4_E2E953BB4A67DC946206EF9D2DA87881=())" (Variables|Default|GetState))))

(fn SaveState
  (params (Save%20Data%20Add%20Add :type S%20Save%20Actor%20Add%20Structure))
  (bind _save_data (|CallParentFunction Save%20Data%20Add%20Add))
  (return _save_data))

(fn LoadState
  (params (SaveDataAdd :type S%20Save%20Actor%20Structure))
  (bind (_position _classactor _isdead _ison _add _actor _baseitem _container _integer) (Utilities|Struct|BreakS_SaveActor SaveDataAdd))
  (|CallParentFunction SaveDataAdd)
  (Transformation|SetActorTransform _position false true)
  (Variables|Default|SetState _integer)
  (CallFunction|UpdateStatus))

(fn UpdateStatus
  (bind _sm1 (Variables|Default|GetSM1))
  (if (== (Variables|Default|GetState) 1)
    (Rendering|SetVisibility (Variables|Default|GetSK2) true false)
    (Components|Animation|PlayAnimation (Variables|Default|GetSK1) "/Game/AnimMeshes/L1_AnimMeshes/Idle.Idle" true)
    (Rendering|SetVisibility _sm1 false false)
    (Collision|SetCollisionEnabled _sm1 "NoCollision")
    (else
      (Rendering|SetVisibility (Variables|Default|GetSK2) false false)
      (Rendering|SetVisibility _sm1 true false)
      (Collision|SetCollisionEnabled _sm1 "QueryAndPhysics"))))