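; BP_Rune_Aam is a saveable magic rune actor that mirrors its TakeRune flag to the player character's Aam value.
; A looping timer started on BeginPlay polls UpdateRune, which hides the mesh and sets Aam when taken, otherwise shows it and clears Aam.
; SaveState and LoadState persist the flag through parent calls, and loading also refreshes the rune.
; Nothing in these graphs sets TakeRune except LoadState.
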(event EventBeginPlay
  (|CallParentFunction)
  (Utilities|Time|SetTimerbyFunctionName 0 "UpdateRune" 0.2 true))

(event Collision|EventActorBeginOverlap
  (params (OtherActor :type Actor%20Object%20Reference))
  (|CallParentFunction OtherActor) ; This node is disabled and will not be called.\nDrag off pins to build functionality.
)

(event EventTick
  (params (DeltaSeconds :type Float%20%28single-precision%29))
  (|CallParentFunction DeltaSeconds) ; This node is disabled and will not be called.\nDrag off pins to build functionality.
)

(fn ConstructionScript
  (|CallParentFunction))

(fn LoadState
  (params (SaveDataAdd :type S%20Save%20Actor%20Structure))
  (|CallParentFunction SaveDataAdd)
  (Variables|Default|SetTakeRune (.IsOn (Utilities|Struct|BreakS_SaveActor SaveDataAdd)))
  (CallFunction|UpdateRune))

(fn UpdateRune
  (bind _mycharacter (CallFunction|--GetPlayerCharacter))
  (bind _staticmesh (Variables|Default|GetStaticMesh))
  (if (Variables|Default|GetTakeRune)
    (Rendering|SetVisibility _staticmesh false false)
    (Variables|/Game/RPGCharacterCreator/Blueprints/BP_RPG_CharacterMain.BP_RPG_CharacterMain_C|SetAam _mycharacter 1)
    (else
      (Rendering|SetVisibility _staticmesh true false)
      (Variables|/Game/RPGCharacterCreator/Blueprints/BP_RPG_CharacterMain.BP_RPG_CharacterMain_C|SetAam _mycharacter 0))))

(fn SaveState
  (params (Save%20Data%20Add%20Add :type S%20Save%20Actor%20Add%20Structure))
  (bind _save_data (|CallParentFunction (Utilities|Struct|MakeS_SaveActorAdd (Utilities|Array|MakeArray (Variables|Default|GetTakeRune)))))
  (return _save_data))

(fn LoadDone
  (|CallParentFunction)
  (CallFunction|UpdateRune))