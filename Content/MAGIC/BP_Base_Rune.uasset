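; Base rune actor that implements interaction and save/load interfaces, likely as a parent for magic runes.
; The interactability check itself sets TakeRune to true and returns it, while interaction only reports success with the name "Руна" (Rune).
; TakeRune is saved as the IsOn flag and restored on load, which also marks the actor Loaded.
; LoadDone and the inventory functions are stubs, and DestroySelf simply destroys the actor.
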(event EventBPILoadDone
  ;[1 1 1] Save/Load
  (CallFunction|LoadDone))

(event Collision|EventActorBeginOverlap
  (params (OtherActor :type Actor%20Object%20Reference)))

(event EventBPILoadState
  (params (SaveSlot :type S%20Save%20Actor%20Structure))
  ;[1 1 1] Save/Load
  (CallFunction|LoadState SaveSlot))

(event EventBeginPlay)

(event EventTick
  (params (DeltaSeconds :type Float%20%28single-precision%29)))

(fn ConstructionScript)

(fn DestroySelf
  (Actor|DestroyActor))

(fn LoadDone
  (if (not (Variables|Default|GetLoaded))
    (return)))

(fn SaveState
  (params (Save%20Data%20Add%20Add :type S%20Save%20Actor%20Add%20Structure))
  (return (Utilities|Struct|MakeS_SaveActor "0.000000,0.000000,0.000000|0.000000,0.000000,0.000000|1.000000,1.000000,1.000000" (Utilities|GetClass self) false (Variables|Default|GetTakeRune) "(BoolArray_2_0C11053C44F85D099D01009D36B474A2=)" self 0 "(Items_4_E2E953BB4A67DC946206EF9D2DA87881=())" 0 0.0)))

(fn LoadState
  (params (SaveDataAdd :type S%20Save%20Actor%20Structure))
  (Variables|Default|SetLoaded true)
  (Variables|Default|SetTakeRune (.ison SaveDataAdd)))

(fn BPISaveState
  (return (Utilities|Struct|MakeS_SaveActor "0.000000,0.000000,0.000000|0.000000,0.000000,0.000000|1.000000,1.000000,1.000000" 0 false (Variables|Default|GetTakeRune))))

(fn ICanbeInteracted
  (bind _output_get (Variables|Default|SetTakeRune true))
  (return _output_get))

(fn IEndInteraction
  (params (InteractingCharacter :type Character%20Object%20Reference))
  (return false))

(fn IGetInteractionText
  (return "" "f"))

(fn IGetInventoryItems
  (return 0))

(fn IInteraction
  (params (InteractingCharacter :type Character%20Object%20Reference))
  (return "Руна" true))

(fn ISetInventoryItems
  (params (Items :type Map%20of%20ST%20Item%20Slot%20Params%20Structures%20to%20Structs))
  (return false))